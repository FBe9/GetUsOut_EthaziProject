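; BP_VRGameMode is a VR game mode that places joining players and sets their hand materials.
; ChoosePlayerStart returns the PlayerStart whose tag matches the current player count.
; Three seconds after BeginPlay, it passes the player count to BP_VRGameState's Postit.
; For three to five players, it also gives each VRPawn except the first a numbered Manny right-hand material, chosen by count and array index.
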(event `self.ReceiveBeginPlay`
  ;[1 1 1] Muestra el numero introducido en el txt correspondiente
  (`KismetSystemLibrary.Delay` 3.0)
  (bind _returnvalue (`self.GetNumPlayers`))
  (bind _asbp_vrgame_state (cast `/Game/Blueprints/BP_VRGameState` (`GameplayStatics.GetGameState`)))
  (`/Game/Blueprints/BP_VRGameState.Postit` _asbp_vrgame_state _returnvalue)
  (bind _outactors (`GameplayStatics.GetAllActorsOfClass` "/Game/VRTemplate/Blueprints/VRPawn.VRPawn_C"))
  (switch `int` _returnvalue
    (:`3`
      (bind _handright (`/Game/VRTemplate/Blueprints/VRPawn.HandRight` (`|GetArrayItem` _outactors 1)))
      (`PrimitiveComponent.SetMaterial` _handright 0 "/Game/Characters/MannequinsXR/Materials/Instances/Manny/MI_Manny_N4.MI_Manny_N4")
      (bind _handright_2 (`/Game/VRTemplate/Blueprints/VRPawn.HandRight` (`|GetArrayItem` _outactors 2)))
      (`PrimitiveComponent.SetMaterial` _handright_2 0 "/Game/Characters/MannequinsXR/Materials/Instances/Manny/MI_Manny_N9.MI_Manny_N9"))
    (:`4`
      (`PrimitiveComponent.SetMaterial` _handright 0 "/Game/Characters/MannequinsXR/Materials/Instances/Manny/MI_Manny_N8.MI_Manny_N8")
      (`PrimitiveComponent.SetMaterial` _handright_2 0 "/Game/Characters/MannequinsXR/Materials/Instances/Manny/MI_Manny_N4.MI_Manny_N4")
      (bind _handright_3 (`/Game/VRTemplate/Blueprints/VRPawn.HandRight` (`|GetArrayItem` _outactors 3)))
      (`PrimitiveComponent.SetMaterial` _handright_3 0 "/Game/Characters/MannequinsXR/Materials/Instances/Manny/MI_Manny_N9.MI_Manny_N9"))
    (:`5`
      (`PrimitiveComponent.SetMaterial` _handright 0 "/Game/Characters/MannequinsXR/Materials/Instances/Manny/MI_Manny_N3.MI_Manny_N3")
      (`PrimitiveComponent.SetMaterial` _handright_2 0 "/Game/Characters/MannequinsXR/Materials/Instances/Manny/MI_Manny_N8.MI_Manny_N8")
      (`PrimitiveComponent.SetMaterial` _handright_3 0 "/Game/Characters/MannequinsXR/Materials/Instances/Manny/MI_Manny_N4.MI_Manny_N4")
      (`PrimitiveComponent.SetMaterial` (`/Game/VRTemplate/Blueprints/VRPawn.HandRight` (`|GetArrayItem` _outactors 4)) 0 "/Game/Characters/MannequinsXR/Materials/Instances/Manny/MI_Manny_N9.MI_Manny_N9"))))

(fn `ChoosePlayerStart`
  (params (Player :type "Controller Object Reference"))
  (returns (ReturnValue :type "Actor Object Reference"))
  (bind _returnvalue (`self.GetNumPlayers`))
  (bind _outactors (`GameplayStatics.GetAllActorsOfClass` "/Script/Engine.PlayerStart"))
  (for _array_element _outactors
    (if (== _returnvalue (`KismetStringLibrary.Conv_NameToString` (`PlayerStart.PlayerStartTag` _array_element)))
      (return _array_element))))

(fn `UserConstructionScript`)
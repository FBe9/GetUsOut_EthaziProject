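; Computer desk Blueprint whose drawers open to reveal puzzle items as the player progresses through levels.
; BeginPlay finds the tagged puzzle cubes and battery by class and tag, relying on fixed array indices, and limits their collision to physics only.
; AbrirCajon slides the top or triangles drawer out depending on SegundoNivel, plays sounds, and enables query collision on that drawer's items, also activating battery physics for the top one.
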(event `AbrirCajon`
  (params (segundoNivel :type Boolean))
  (bind _v001_mesilla_cajon_cajon_arriba (`self.v001_Mesilla_Cajon_Cajon_Arriba`))
  (bind _v001_mesilla_cajon_cajon_triangulos (`self.v001_Mesilla_Cajon_Cajon_triangulos`))
  (bind (_relativelocation_x _relativelocation_y _relativelocation_z) (`KismetMathLibrary.BreakVector` (`SceneComponent.RelativeLocation` _v001_mesilla_cajon_cajon_triangulos)))
  (bind (_relativelocation_x_2 _relativelocation_y_2 _relativelocation_z_2) (`KismetMathLibrary.BreakVector` (`SceneComponent.RelativeLocation` _v001_mesilla_cajon_cajon_arriba)))
  ;[1 1 1] Abre los cajones del ordenador segun el nivel
  (if segundoNivel
    (`KismetSystemLibrary.MoveComponentTo` _v001_mesilla_cajon_cajon_triangulos (`KismetMathLibrary.MakeVector` -30.0 _relativelocation_y _relativelocation_z) (struct) false false 1.0)
    (`GameplayStatics.PlaySound2D` "/Game/Audio/Audio_AbrirCajon_Caja_Puzle.Audio_AbrirCajon_Caja_Puzle" 1.0 1.0 0.0 null null)
    (`GameplayStatics.PlaySound2D` "/Game/Audio/AudiosPshicopat/Ordenador-2.Ordenador-2" 1.0 1.0 0.0 null null)
    (`PrimitiveComponent.SetCollisionEnabled` (`/Game/Blueprints/Caja_Puzle/BP_Cubo_Puzle.StaticMesh` (`self.BP_Cubo2`)) "QueryAndPhysics")
    (else
      (`PrimitiveComponent.SetSimulatePhysics` (`/Game/Blueprints/Mando_Pilas/BP_Pila.Pila` (`self.BP_Pila`)) true)
      (`KismetSystemLibrary.MoveComponentTo` _v001_mesilla_cajon_cajon_arriba (`KismetMathLibrary.MakeVector` -30.0 _relativelocation_y_2 _relativelocation_z_2) (struct) false false 1.0)
      (`GameplayStatics.PlaySound2D` "/Game/Audio/Audio_AbrirCajon_Caja_Puzle.Audio_AbrirCajon_Caja_Puzle" 1.0 1.0 0.0 null null)
      (`PrimitiveComponent.SetCollisionEnabled` (`/Game/Blueprints/Caja_Puzle/BP_Cubo_Puzle.StaticMesh` (`self.BP_Cubo`)) "QueryAndPhysics")
      (`PrimitiveComponent.SetCollisionEnabled` (`/Game/Blueprints/Mando_Pilas/BP_Pila.Pila` (`self.BP_Pila`)) "QueryAndPhysics")
      (`GameplayStatics.PlaySound2D` "/Game/Audio/AudiosPshicopat/Tercer-Paso.Tercer-Paso" 1.0 1.0 0.0 null null))))

(event `self.ReceiveBeginPlay`
  ;[1 1 1] REcoje los cubos y las pilas en sus variables
  (bind _outactors (`GameplayStatics.GetAllActorsOfClassWithTag` "/Game/Blueprints/Caja_Puzle/BP_Cubo_Puzle.BP_Cubo_Puzle_C" "1"))
  (bind _output_get (set `self.BP_Cubo` (`|GetArrayItem` _outactors 2)))
  (`PrimitiveComponent.SetCollisionEnabled` (`/Game/Blueprints/Caja_Puzle/BP_Cubo_Puzle.StaticMesh` _output_get) "PhysicsOnly")
  (bind _outactors_2 (`GameplayStatics.GetAllActorsOfClassWithTag` "/Game/Blueprints/Mando_Pilas/BP_Pila.BP_Pila_C" "pila1"))
  (bind _output_get_2 (set `self.BP_Pila` (`|GetArrayItem` _outactors_2)))
  (`PrimitiveComponent.SetCollisionEnabled` (`/Game/Blueprints/Mando_Pilas/BP_Pila.Pila` _output_get_2) "PhysicsOnly")
  (bind _outactors_3 (`GameplayStatics.GetAllActorsOfClassWithTag` "/Game/Blueprints/Caja_Puzle/BP_Cubo_Puzle.BP_Cubo_Puzle_C" "2"))
  (bind _output (`|GetArrayItem` _outactors_3 1))
  (set `self.BP_Cubo2` _output)
  (`PrimitiveComponent.SetCollisionEnabled` (`/Game/Blueprints/Caja_Puzle/BP_Cubo_Puzle.StaticMesh` _output) "PhysicsOnly"))

(fn `UserConstructionScript`)
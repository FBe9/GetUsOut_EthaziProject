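; BP_Booth is a five-button color puzzle that opens a booth barrier and reveals a probeta.
; Each overlap cycles that button's counter through five cable materials, with timelines animating the press and return while a shared Clicked flag blocks other presses.
; Every press compares the counters to Colors, where button five reuses the first entry.
; A match hides the barrier, enables the fourth BP_Probeta found in the level, and plays a sound.
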(event `self.LAB_to_UE_Button_1.OnComponentBeginOverlap`
  (params (OverlappedComponent :type "PrimitiveComponent Object Reference") (OtherActor :type "Actor Object Reference") (OtherComp :type "PrimitiveComponent Object Reference") (OtherBodyIndex :type Integer) (bFromSweep :type Boolean) (SweepResult :type "HitResult Structure (by ref)"))
  (bind _colorbutton1 (`self.ColorButton1`))
  (if (not (`self.Clicked`))
    (set `self.Clicked` true)
    (`self.ButtonGoingDown` (`self.LAB_to_UE_Button_1`))
    (`/Engine/EditorBlueprintResources/StandardMacros.IncrementInt` (`self.ColorButton1`)
      (:`  `
        (if (== _colorbutton1 5)
          (set `self.ColorButton1` 0)
          (`PrimitiveComponent.SetMaterial` (`self.LAB_to_UE_Button_1`) 0 "/Game/Blueprints/BombaYBoton/MI_Cable_1.MI_Cable_1")
          (`self.Check Colors and Open Door` :!label _label)
          (elif (== _colorbutton1 1)
            (`PrimitiveComponent.SetMaterial` (`self.LAB_to_UE_Button_1`) 0 "/Game/Blueprints/BombaYBoton/MI_Cable_2.MI_Cable_2")
            (goto _label)
            (elif (== _colorbutton1 2)
              (`PrimitiveComponent.SetMaterial` (`self.LAB_to_UE_Button_1`) 0 "/Game/Blueprints/BombaYBoton/MI_Cable_3.MI_Cable_3")
              (goto _label)
              (elif (== _colorbutton1 3)
                (`PrimitiveComponent.SetMaterial` (`self.LAB_to_UE_Button_1`) 0 "/Game/Blueprints/BombaYBoton/MI_Cable_4.MI_Cable_4")
                (goto _label)
                (elif (== _colorbutton1 4)
                  (`PrimitiveComponent.SetMaterial` (`self.LAB_to_UE_Button_1`) 0 "/Game/Blueprints/BombaYBoton/MI_Cable_5.MI_Cable_5")
                  (goto _label))))))))))

(event `self.LAB_to_UE_Button_2.OnComponentBeginOverlap`
  (params (OverlappedComponent :type "PrimitiveComponent Object Reference") (OtherActor :type "Actor Object Reference") (OtherComp :type "PrimitiveComponent Object Reference") (OtherBodyIndex :type Integer) (bFromSweep :type Boolean) (SweepResult :type "HitResult Structure (by ref)"))
  (bind _colorbutton2 (`self.ColorButton2`))
  (bind _lab_to_ue_button_2 (`self.LAB_to_UE_Button_2`))
  (if (not (`self.Clicked`))
    (set `self.Clicked` true)
    (`self.ButtonGoingDown` (`self.LAB_to_UE_Button_2`))
    (`/Engine/EditorBlueprintResources/StandardMacros.IncrementInt` _colorbutton2
      (:`  `
        (if (== _colorbutton2 5)
          (set `self.ColorButton2` 0)
          (`PrimitiveComponent.SetMaterial` _lab_to_ue_button_2 0 "/Game/Blueprints/BombaYBoton/MI_Cable_1.MI_Cable_1")
          (`self.Check Colors and Open Door` :!label _label_2)
          (elif (== _colorbutton2 1)
            (`PrimitiveComponent.SetMaterial` _lab_to_ue_button_2 0 "/Game/Blueprints/BombaYBoton/MI_Cable_2.MI_Cable_2")
            (goto _label_2)
            (elif (== _colorbutton2 2)
              (`PrimitiveComponent.SetMaterial` _lab_to_ue_button_2 0 "/Game/Blueprints/BombaYBoton/MI_Cable_3.MI_Cable_3")
              (goto _label_2)
              (elif (== _colorbutton2 3)
                (`PrimitiveComponent.SetMaterial` _lab_to_ue_button_2 0 "/Game/Blueprints/BombaYBoton/MI_Cable_5.MI_Cable_5")
                (goto _label_2)
                (elif (== _colorbutton2 4)
                  (`PrimitiveComponent.SetMaterial` _lab_to_ue_button_2 0 "/Game/Blueprints/BombaYBoton/MI_Cable_6.MI_Cable_6")
                  (goto _label_2))))))))))

(event `self.LAB_to_UE_Button_3.OnComponentBeginOverlap`
  (params (OverlappedComponent :type "PrimitiveComponent Object Reference") (OtherActor :type "Actor Object Reference") (OtherComp :type "PrimitiveComponent Object Reference") (OtherBodyIndex :type Integer) (bFromSweep :type Boolean) (SweepResult :type "HitResult Structure (by ref)"))
  (bind _lab_to_ue_button_3 (`self.LAB_to_UE_Button_3`))
  (bind _colorbutton3 (`self.ColorButton3`))
  (if (not (`self.Clicked`))
    (set `self.Clicked` true)
    (`self.ButtonGoingDown` (`self.LAB_to_UE_Button_3`))
    (`/Engine/EditorBlueprintResources/StandardMacros.IncrementInt` _colorbutton3
      (:`  `
        (if (== _colorbutton3 5)
          (set `self.ColorButton3` 0)
          (`PrimitiveComponent.SetMaterial` _lab_to_ue_button_3 0 "/Game/Blueprints/BombaYBoton/MI_Cable_1.MI_Cable_1")
          (`self.Check Colors and Open Door` :!label _label_3)
          (elif (== _colorbutton3 1)
            (`PrimitiveComponent.SetMaterial` _lab_to_ue_button_3 0 "/Game/Blueprints/BombaYBoton/MI_Cable_2.MI_Cable_2")
            (goto _label_3)
            (elif (== _colorbutton3 2)
              (`PrimitiveComponent.SetMaterial` _lab_to_ue_button_3 0 "/Game/Blueprints/BombaYBoton/MI_Cable_3.MI_Cable_3")
              (goto _label_3)
              (elif (== _colorbutton3 3)
                (`PrimitiveComponent.SetMaterial` _lab_to_ue_button_3 0 "/Game/Blueprints/BombaYBoton/MI_Cable_4.MI_Cable_4")
                (goto _label_3)
                (elif (== _colorbutton3 4)
                  (`PrimitiveComponent.SetMaterial` _lab_to_ue_button_3 0 "/Game/Blueprints/BombaYBoton/MI_Cable_5.MI_Cable_5")
                  (goto _label_3))))))))))

(event `self.LAB_to_UE_Button_4.OnComponentBeginOverlap`
  (params (OverlappedComponent :type "PrimitiveComponent Object Reference") (OtherActor :type "Actor Object Reference") (OtherComp :type "PrimitiveComponent Object Reference") (OtherBodyIndex :type Integer) (bFromSweep :type Boolean) (SweepResult :type "HitResult Structure (by ref)"))
  (bind _colorbutton4 (`self.ColorButton4`))
  (bind _lab_to_ue_button_4 (`self.LAB_to_UE_Button_4`))
  (if (not (`self.Clicked`))
    (set `self.Clicked` true)
    (`self.ButtonGoingDown` (`self.LAB_to_UE_Button_4`))
    (`/Engine/EditorBlueprintResources/StandardMacros.IncrementInt` _colorbutton4
      (:`  `
        (if (== _colorbutton4 5)
          (set `self.ColorButton4` 0)
          (`PrimitiveComponent.SetMaterial` _lab_to_ue_button_4 0 "/Game/Blueprints/BombaYBoton/MI_Cable_1.MI_Cable_1")
          (`self.Check Colors and Open Door` :!label _label_4)
          (elif (== _colorbutton4 1)
            (`PrimitiveComponent.SetMaterial` _lab_to_ue_button_4 0 "/Game/Blueprints/BombaYBoton/MI_Cable_2.MI_Cable_2")
            (goto _label_4)
            (elif (== _colorbutton4 2)
              (`PrimitiveComponent.SetMaterial` _lab_to_ue_button_4 0 "/Game/Blueprints/BombaYBoton/MI_Cable_3.MI_Cable_3")
              (goto _label_4)
              (elif (== _colorbutton4 3)
                (`PrimitiveComponent.SetMaterial` _lab_to_ue_button_4 0 "/Game/Blueprints/BombaYBoton/MI_Cable_4.MI_Cable_4")
                (goto _label_4)
                (elif (== _colorbutton4 4)
                  (`PrimitiveComponent.SetMaterial` _lab_to_ue_button_4 0 "/Game/Blueprints/BombaYBoton/MI_Cable_5.MI_Cable_5")
                  (goto _label_4))))))))))

(event `SpawnProbeta`
  ;[1 1 1] Spawn Probeta Morada
  (bind _outactors (`GameplayStatics.GetAllActorsOfClass` "/Game/Blueprints/Probetas/BP_Probeta.BP_Probeta_C"))
  (bind _output (`|GetArrayItem` _outactors 3))
  (`SceneComponent.SetVisibility` (`Actor.RootComponent` _output) true false)
  (bind _staticmesh (`/Game/Blueprints/Probetas/BP_Probeta.StaticMesh` _output))
  (`PrimitiveComponent.SetCollisionEnabled` _staticmesh "QueryAndPhysics")
  (`PrimitiveComponent.SetSimulatePhysics` _staticmesh true)
  (`GameplayStatics.PlaySound2D` "/Game/Audio/AudiosPshicopat/Lab/Botones_Colores.Botones_Colores" 1.0 1.0 0.0 null null))

(event `self.LAB_to_UE_Button_5.OnComponentBeginOverlap`
  (params (OverlappedComponent :type "PrimitiveComponent Object Reference") (OtherActor :type "Actor Object Reference") (OtherComp :type "PrimitiveComponent Object Reference") (OtherBodyIndex :type Integer) (bFromSweep :type Boolean) (SweepResult :type "HitResult Structure (by ref)"))
  (bind _lab_to_ue_button_5 (`self.LAB_to_UE_Button_5`))
  (bind _colorbutton5 (`self.ColorButton5`))
  (if (not (`self.Clicked`))
    (set `self.Clicked` true)
    (`self.ButtonGoingDown` (`self.LAB_to_UE_Button_5`))
    (`/Engine/EditorBlueprintResources/StandardMacros.IncrementInt` _colorbutton5
      (:`  `
        (if (== _colorbutton5 5)
          (set `self.ColorButton5` 0)
          (`PrimitiveComponent.SetMaterial` _lab_to_ue_button_5 0 "/Game/Blueprints/BombaYBoton/MI_Cable_1.MI_Cable_1")
          (`self.Check Colors and Open Door` :!label _label_5)
          (elif (== _colorbutton5 1)
            (`PrimitiveComponent.SetMaterial` _lab_to_ue_button_5 0 "/Game/Blueprints/BombaYBoton/MI_Cable_2.MI_Cable_2")
            (goto _label_5)
            (elif (== _colorbutton5 2)
              (`PrimitiveComponent.SetMaterial` _lab_to_ue_button_5 0 "/Game/Blueprints/BombaYBoton/MI_Cable_3.MI_Cable_3")
              (goto _label_5)
              (elif (== _colorbutton5 3)
                (`PrimitiveComponent.SetMaterial` _lab_to_ue_button_5 0 "/Game/Blueprints/BombaYBoton/MI_Cable_4.MI_Cable_4")
                (goto _label_5)
                (elif (== _colorbutton5 4)
                  (`PrimitiveComponent.SetMaterial` _lab_to_ue_button_5 0 "/Game/Blueprints/BombaYBoton/MI_Cable_5.MI_Cable_5")
                  (goto _label_5))))))))))

(event `ButtonGoingDown`
  (params (Button :type "SceneComponent Object Reference (by ref)"))
  ;[1 1 1] ButtonGoingDown
  (`self.SetInitialAndFinalLocations` Button)
  (bind (_direction _newtrack_0) (`Timeline|Timeline` :!via `PlayFromStart`)
    (:`Update`
      (`SceneComponent.K2_SetWorldLocation` Button (`KismetMathLibrary.VLerp` (`self.InitialLocation`) (`self.FinalLocation`) _newtrack_0) false false))
    (:`Finished`
      ;[1 1 1] ButtonGoingUp
      (bind (_direction_2 _newtrack_0_2) (`Timeline|Timeline_0` :!via `ReverseFromEnd`)
        (:`Update`
          (`SceneComponent.K2_SetWorldLocation` Button (`KismetMathLibrary.VLerp` (`self.InitialLocation`) (`self.FinalLocation`) _newtrack_0_2) false false))
        (:`Finished`
          (set `self.Clicked` false))))))

(fn `Check Colors and Open Door`
  (bind _lab_to_ue_booth_barrera (`self.LAB_to_UE_Booth_Barrera`))
  (bind _colors (`self.Colors`))
  (if (and (== (`|GetArrayItem` _colors) (`self.ColorButton1`)) (== (`|GetArrayItem` _colors 1) (`self.ColorButton2`)) (== (`|GetArrayItem` _colors 2) (`self.ColorButton3`)) (== (`|GetArrayItem` _colors 3) (`self.ColorButton4`)) (== (`|GetArrayItem` _colors) (`self.ColorButton5`)))
    (`SceneComponent.SetVisibility` _lab_to_ue_booth_barrera false false)
    (`PrimitiveComponent.SetCollisionEnabled` _lab_to_ue_booth_barrera "NoCollision")
    (`self.SpawnProbeta`)))

(fn `SetInitialAndFinalLocations`
  (params (Button :type "SceneComponent Object Reference"))
  (bind _output_get (set `self.InitialLocation` (`SceneComponent.K2_GetComponentLocation` Button)))
  (set `self.FinalLocation` (`KismetMathLibrary.MakeVector` (- (.x _output_get) 0.5) (.y _output_get) (- (.z _output_get) 1.0))))

(fn `UserConstructionScript`)
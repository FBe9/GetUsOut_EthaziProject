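; VR push button for a puzzle where two BP_BotonClick buttons must be pressed at the same time to reveal a test tube (Probeta).
; VRPawn overlap sets BotonPulsado and plays timelines that lower and raise the mesh, clearing the flag during the rise.
; When the first two button instances are both pressed, it shows the third BP_Probeta found, enables its collision and physics, and plays a sound.
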(event `self.ReceiveBeginPlay`
  ;[1 1 1] Set Location
  (bind _output_get (set `self.InitialLocation` (`SceneComponent.K2_GetComponentLocation` (`self.StaticMesh`))))
  (set `self.EndLocation` (`KismetMathLibrary.MakeVector` (.x _output_get) (.y _output_get) (- (.z _output_get) 2.5))))

(event `Bajar_Boton`
  ;[1 1 1] Bajar Boton
  (bind (_direction _newtrack_0) (`Timeline|Timeline_1` :!via `PlayFromStart`)
    (:`Update`
      (`SceneComponent.K2_SetWorldLocation` (`self.StaticMesh`) (`KismetMathLibrary.VLerp` (`self.InitialLocation`) (`self.EndLocation`) _newtrack_0) false false))
    (:`Finished`
      (`self.Subir_boton`))))

(event `Subir_boton`
  ;[1 1 1] Subir Boton
  (bind (_direction _newtrack_0) (`Timeline|Timeline_2` :!via `ReverseFromEnd`)
    (:`Update`
      (`SceneComponent.K2_SetWorldLocation` (`self.StaticMesh`) (`KismetMathLibrary.VLerp` (`self.InitialLocation`) (`self.EndLocation`) _newtrack_0) false false)
      (set `self.BotonPulsado` false))))

(event `self.ReceiveActorBeginOverlap`
  (params (OtherActor :type "Actor Object Reference"))
  ;[1 1 1] CheckSummonedYPursado
  (cast `/Game/VRTemplate/Blueprints/VRPawn` OtherActor)
  (if (not (`self.ProbetaSummoned`))
    (set `self.BotonPulsado` true)
    (bind _outactors (`GameplayStatics.GetAllActorsOfClass` "BP_BotonClick_C"))
    (if (and (`/Game/Blueprints/BotonesAlaVez/BP_BotonClick.BotonPulsado` (`|GetArrayItem` _outactors)) (`/Game/Blueprints/BotonesAlaVez/BP_BotonClick.BotonPulsado` (`|GetArrayItem` _outactors 1)))
      (`self.Bajar_Boton`)
      (`self.SpawnProbeta`)
      (else
        (`self.Bajar_Boton`)))))

(event `SpawnProbeta`
  ;[1 1 1] SpawnProbetaVerde
  (set `self.ProbetaSummoned` true)
  (bind _outactors (`GameplayStatics.GetAllActorsOfClass` "/Game/Blueprints/Probetas/BP_Probeta.BP_Probeta_C"))
  (bind _output (`|GetArrayItem` _outactors 2))
  (`SceneComponent.SetVisibility` (`Actor.RootComponent` _output) true false)
  (bind _staticmesh (`/Game/Blueprints/Probetas/BP_Probeta.StaticMesh` _output))
  (`PrimitiveComponent.SetCollisionEnabled` _staticmesh "QueryAndPhysics")
  (`PrimitiveComponent.SetSimulatePhysics` _staticmesh true)
  (`GameplayStatics.PlaySound2D` "/Game/Audio/AudiosPshicopat/Lab/Botones_dobles.Botones_dobles" 1.0 1.0 0.0 null null))

(fn `UserConstructionScript`)
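; BP_btonLuz is a light switch actor that toggles the lamps in the level whenever any actor begins overlapping it.
; Each overlap flips its Encendido state, tilts the button mesh to match, and plays the ApagarLuces sound only the first time.
; It then finds every BP_Lampara, inverts each lamp's own Encendido flag, and sets its PointLight visibility from it, so lamps toggle independently of the switch state.
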(event `self.ReceiveActorBeginOverlap`
  (params (OtherActor :type "Actor Object Reference"))
  (bind _interruptor_interruptor_boton (`self.Interruptor_Interruptor_Boton`))
  ;[1 1 1] Encendido y apagado de la luz
  (if (`self.firstTime`)
    (set `self.firstTime` false)
    (`GameplayStatics.PlaySound2D` "/Game/Audio/AudiosPshicopat/Apagar-Luces.Apagar-Luces" 1.0 1.0 0.0 null null))
  (bind _output_get (set `self.Encendido` (not (`self.Encendido`))))
  (if _output_get
    (`SceneComponent.K2_SetRelativeRotation` _interruptor_interruptor_boton (struct :`Pitch` 4.883549) false false)
    (else
      (`SceneComponent.K2_SetRelativeRotation` _interruptor_interruptor_boton (struct :`Pitch` -7.0) false false)))
  (bind _outactors (`GameplayStatics.GetAllActorsOfClass` "/Game/Blueprints/Interruptor/BP_Lampara.BP_Lampara_C"))
  (for _array_element _outactors
    (bind _output_get_2 (set `/Game/Blueprints/Interruptor/BP_Lampara.Encendido` (not (`/Game/Blueprints/Interruptor/BP_Lampara.Encendido` _array_element)) _array_element))
    (`SceneComponent.SetVisibility` (`/Game/Blueprints/Interruptor/BP_Lampara.PointLight` _array_element) _output_get_2 false)))

(fn `UserConstructionScript`)
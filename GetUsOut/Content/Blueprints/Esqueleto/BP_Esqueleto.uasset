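; BP_Esqueleto is a skeleton puzzle piece that accepts a missing rib and reveals a test tube as a result.
; When a BP_CostillaEsqueleto overlaps its Box, it destroys that actor and shows the skeleton's own hidden rib component.
; It then calls SpawnProbeta, which spawns nothing but makes an existing BP_Probeta (the purple one) visible with collision and physics.
; That tube is picked by hardcoded index from GetAllActorsOfClass, so it depends on actor order.
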(event `self.Box.OnComponentBeginOverlap`
  (params (OverlappedComponent :type "PrimitiveComponent Object Reference") (OtherActor :type "Actor Object Reference") (OtherComp :type "PrimitiveComponent Object Reference") (OtherBodyIndex :type Integer) (bFromSweep :type Boolean) (SweepResult :type "HitResult Structure (by ref)"))
  ;[1 1 1] Box on component begin overlab | Hacer Visible Costilla
  (bind _asbp_costilla_esqueleto (cast `/Game/Blueprints/Esqueleto/BP_CostillaEsqueleto` OtherActor))
  (`self.K2_DestroyActor` _asbp_costilla_esqueleto)
  (`SceneComponent.SetVisibility` (`self.Esqueleto_Esqueleto_Costilla`) true false)
  (`self.SpawnProbeta`))

(event `SpawnProbeta`
  ;[1 1 1] Spawn Probeta Morada
  (bind _outactors (`GameplayStatics.GetAllActorsOfClass` "/Game/Blueprints/Probetas/BP_Probeta.BP_Probeta_C"))
  (bind _output (`|GetArrayItem` _outactors 1))
  (`SceneComponent.SetVisibility` (`Actor.RootComponent` _output) true false)
  (bind _staticmesh (`/Game/Blueprints/Probetas/BP_Probeta.StaticMesh` _output))
  (`PrimitiveComponent.SetCollisionEnabled` _staticmesh "QueryAndPhysics")
  (`PrimitiveComponent.SetSimulatePhysics` _staticmesh true))

(fn `UserConstructionScript`)
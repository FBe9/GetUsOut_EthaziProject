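; Lobby player controller that gives host and clients their session screens and tracks each player's icon and ready state.
; Host gets a screen with Start disabled; clients get a screen plus a spawned MenuClientLobby actor, whose widget receives list updates.
; Player icon comes from IconTable via the GameInstance's choice, with clients sending it by RPC.
; Ready toggles notify the lobby GameMode.
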(event `CreateWidget`
  ;[1 1 1] Crea los widget correspondientes del host o del client uando entren a la sesion
  (`/Engine/EditorBlueprintResources/ActorMacros.Switch Has Authority`
    (:`Authority`
      (bind _returnvalue (`|CreateWidget` "/Game/Widgets/WidgetsLobby/WID_HostScreen.WID_HostScreen_C"))
      (`UserWidget.AddToViewport` _returnvalue 0)
      (set `self.LobbyWidget` _returnvalue)
      (set `Widget.bIsEnabled` false (`/Game/Widgets/WidgetsLobby/WID_HostScreen.btn_Start` _returnvalue)))
    (:`Remote`
      (bind _returnvalue_2 (`|CreateWidget` "/Game/Widgets/WidgetsLobby/WID_ClientScreen.WID_ClientScreen_C"))
      (`UserWidget.AddToViewport` _returnvalue_2 0)
      (bind _returnvalue_3 (`GameplayStatics.GetActorOfClass` "/Game/VRTemplate/Blueprints/VRPawn.VRPawn_C"))
      (bind _returnvalue_4 (`|SpawnActorFromClass` "/Game/Widgets/BlueprintsLobby/MenuClientLobby.MenuClientLobby_C" (`KismetMathLibrary.MakeTransform` (0.0 0.0 0.0)) "Undefined" "MultiplyWithRoot" null false _returnvalue_3))
      (bind _aswid_client_screen (cast `/Game/Widgets/WidgetsLobby/WID_ClientScreen` (`WidgetComponent.GetWidget` (`/Game/Widgets/BlueprintsLobby/MenuClientLobby.Widget` _returnvalue_4)))
        (:`then`
          (set `self.LobbyWidget` _aswid_client_screen))
        (:`CastFailed`
          (`KismetSystemLibrary.PrintString` "NO" true true (struct :`R` 0.326494 :`G` 1.0 :`B` 0.095488 :`A` 1.0) 50.0))))))

(event `UpdatePlayerList`
  (params (PlayerInfo :type "Array of /Game/Widgets/BlueprintsLobby/PlayerInfo Structure (by ref)"))
  (bind _lobbywidget (`self.LobbyWidget`))
  ;[1 1 1] Actualiza la lista de jugadores de los widget del host y del client
  (`/Engine/EditorBlueprintResources/ActorMacros.Switch Has Authority`
    (:`Authority`
      (bind _aswid_host_screen (cast `/Game/Widgets/WidgetsLobby/WID_HostScreen` _lobbywidget)
        (:`then`
          (`/Game/Widgets/WidgetsLobby/WID_HostScreen.UpdatePlayerList` _aswid_host_screen PlayerInfo))
        (:`CastFailed`
          (`KismetSystemLibrary.PrintString` "Cast failed WID_ClientScreen or WID_HostScreen" :!label _label))))
    (:`Remote`
      (bind _aswid_client_screen (cast `/Game/Widgets/WidgetsLobby/WID_ClientScreen` _lobbywidget)
        (:`then`
          (`/Game/Widgets/WidgetsLobby/WID_ClientScreen.UpdatePlayerList` _aswid_client_screen PlayerInfo))
        (:`CastFailed`
          (goto _label))))))

(event `UpdatePlayerInfo`
  ;[1 1 1] Actualiza la informacion de los jugadores cuando entren a la sesion
  (bind _asbp_game_instance (cast `/Game/Blueprints/Lobby/Blueprint/BP_GameInstance` (`GameplayStatics.GetGameInstance`)))
  (bind _returnvalue (`|GetDataTableRow` "/Game/Widgets/BlueprintsMainMenu/IconTable.IconTable" (`KismetStringLibrary.Conv_StringToName` (`/Game/Blueprints/Lobby/Blueprint/BP_GameInstance.IconoJugador` _asbp_game_instance)))
    (:`then`
      (`/Engine/EditorBlueprintResources/ActorMacros.Switch Has Authority`
        (:`Authority`
          (set `self.PlayerInfo` (make `/Game/Widgets/BlueprintsLobby/PlayerInfo` false)))
        (:`Remote`
          (`self.RPC_UpdatePlayerInfo` (`.Icono_5_192070FD46B8849C92DD18A96B4D3146` (break `/Game/Widgets/BlueprintsMainMenu/Iconos` _returnvalue))))))))

(event `RPC_UpdatePlayerInfo`
  (params (`Player Info Player Icon` :type "Texture2D Object Reference") (`Player Info Player Name` :type String))
  ;[1 1 1] Actualiza la informacion de los jugadores cuando entren a la sesion
  (set `self.PlayerInfo` (make `/Game/Widgets/BlueprintsLobby/PlayerInfo` false)))

(event `UpdateStatus`
  (bind _playerinfo_isready (break `/Game/Widgets/BlueprintsLobby/PlayerInfo` (`self.PlayerInfo`)))
  ;[1 1 1] Actualiza si los jugadores están listos o no
  (set `self.PlayerInfo` (make `/Game/Widgets/BlueprintsLobby/PlayerInfo` (not _playerinfo_isready)))
  (bind _asbp_lobby_game_mode_base (cast `/Game/Blueprints/Lobby/Blueprint/BP_LobbyGameModeBase` (`GameplayStatics.GetGameMode`)))
  (`/Game/Blueprints/Lobby/Blueprint/BP_LobbyGameModeBase.UpdateStatus` _asbp_lobby_game_mode_base))

(fn `UserConstructionScript`)
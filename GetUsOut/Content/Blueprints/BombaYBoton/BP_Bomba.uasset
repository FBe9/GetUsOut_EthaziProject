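; BP_Bomba is a bomb actor with a countdown that the player defuses through correct inputs.
; BombaSube moves it to a fixed raised position, then after a delay starts a timer calling BombTimer to decrement TimerBomb.
; Error subtracts a time penalty, and Correct counts successes until it disarms the bomb by clearing the Looping flag.
; When time runs out, Explosion destroys the actor, plays sound and also calls TimerStart again.
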(event `TimerStart`
  (bind _returnvalue (`KismetSystemLibrary.K2_SetTimer` null "BombTimer" 1.0 (`self.Looping`)))
  (set `self.Timer` _returnvalue))

(event `BombaSube`
  ;[1 0 0] ALTURA CON LA BOMBA = 149
  (`self.K2_SetActorLocation` (0.0 0.0 149.0))
  (`GameplayStatics.PlaySound2D` "/Game/Audio/AudiosPshicopat/Lab/Salida_de_Bomba.Salida_de_Bomba" 1.0 1.0 0.0 null null)
  (`KismetSystemLibrary.Delay` 6.0)
  (`self.TimerStart`))

(fn `BombTimer`
  ;[1 1 1] Temporizador - Game Mode
  (if (`self.Looping`)
    (if (>= (`self.TimerBomb`) 0)
      (`/Engine/EditorBlueprintResources/StandardMacros.DecrementInt` (`self.TimerBomb`)
        (:`  `
          (bind _output_get (set `self.TimerBomb` (`self.TimerBomb`)))
          (if (<= _output_get 0)
            (`self.Explosion`)))))))

(fn `Correct`
  (bind _correctnumber (`self.CorrectNumber`))
  (`/Engine/EditorBlueprintResources/StandardMacros.IncrementInt` _correctnumber
    (:`  `
      (if (>= _correctnumber 5)
        (`KismetSystemLibrary.PrintString` "Desactivado")
        (set `self.Looping` false)
        (`GameplayStatics.PlaySound2D` "/Game/Audio/AudiosPshicopat/Lab/Evaluar__bomba_no_boom_boom_.Evaluar__bomba_no_boom_boom_" 1.0 1.0 0.0 null null)))))

(fn `Error`
  (if (`self.Looping`)
    (bind _output_get (set `self.TimerBomb` (- (`self.TimerBomb`) 5)))
    (`GameplayStatics.PlaySoundAtLocation` "/Engine/EngineSounds/1kSineTonePing.1kSineTonePing" (`self.K2_GetActorLocation`) (struct) 1.0 1.0 0.0 null null null null)
    (if (<= _output_get 0)
      (`self.Explosion`))))

(fn `Explosion`
  (`KismetSystemLibrary.PrintString` "LUL U DEAD")
  (`self.K2_DestroyActor`)
  (`GameplayStatics.PlaySoundAtLocation` null (`self.K2_GetActorLocation`) (struct) 1.0 1.0 0.0 null null null null)
  (`self.TimerStart`)
  (`GameplayStatics.PlaySound2D` "/Game/Audio/AudiosPshicopat/Lab/Bomba_Explotifa.Bomba_Explotifa" 1.0 1.0 0.0 null null))

(fn `UserConstructionScript`)
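; Basement door Blueprint that opens once and, when both doors are open, moves the game on to the laboratory level.
; AbrirPuerta sets the Open flag, plays a sound, starts the door mesh rotating and calls ComprobarPuertas.
; That check reads the first two door actors tagged "Puerta"; if both are open, it plays a transition sound, streams in Laboratorio and unloads SotanoFinal after a delay.
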(event `AbrirPuerta`
  ;[1 1 1] Abrir Puerta
  (if (not (`self.open`))
    (set `self.open` true)
    (`GameplayStatics.PlaySound2D` "/Game/Audio/Audio_PuertaAbriendose2Mitad.Audio_PuertaAbriendose2Mitad" 1.0 1.0 0.0 null null)
    (`KismetSystemLibrary.MoveComponentTo` (`self.Sotano_Puerta_Door_004`) (0.0 0.0 0.0) (struct :`Yaw` -140.0) false false 2.0)
    (`self.ComprobarPuertas`)))

(event `ComprobarPuertas`
  ;[1 1 1] Comprobar para mandar al lab
  (bind _outactors (`GameplayStatics.GetAllActorsOfClassWithTag` "BP_PuertaSotano_C" "Puerta"))
  (if (and (`/Game/SotanoFInal/BP_PuertaSotano.open` (`|GetArrayItem` _outactors)) (`/Game/SotanoFInal/BP_PuertaSotano.open` (`|GetArrayItem` _outactors 1)))
    (`GameplayStatics.PlaySound2D` "/Game/Audio/AudiosPshicopat/Transición_.Transición_" 1.0 1.0 0.0 null null)
    (`GameplayStatics.LoadStreamLevelBySoftObjectPtr` "/Game/Levels/Laboratorio.Laboratorio" true)
    (`KismetSystemLibrary.Delay` 10.0)
    (`GameplayStatics.UnloadStreamLevelBySoftObjectPtr` "/Game/Levels/SotanoFinal.SotanoFinal")))

(fn `UserConstructionScript`)
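; Pressure plate that sinks under a BP_Daruma and opens a basement door when the Daruma's first tag matches the plate's.
; The door is one of the first two BP_PuertaSotano tagged "Puerta": the first if its tag matches, otherwise the second, unchecked.
; Two timelines lerp the plate base down and back from its current position.
; Any end overlap raises the plate and permanently shifts its collision box slightly lower.
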(event `self.ReceiveBeginPlay`
  ;[1 1 1] SetLocation
  (bind _output_get (set `self.StartLocation` (`SceneComponent.K2_GetComponentLocation` (`self.PlataformaPlaca`))))
  (set `self.CollisionLocation` (`SceneComponent.K2_GetComponentLocation` (`self.Box`)))
  (set `self.CurrentLocation` _output_get))

(event `self.ReceiveActorBeginOverlap`
  (params (OtherActor :type "Actor Object Reference"))
  ;[1 1 1] Overlap
  (bind _asbp_daruma (cast `/Game/Blueprints/Daruma/BP_Daruma` OtherActor))
  (bind _output (`|GetArrayItem` (`Actor.Tags` _asbp_daruma)))
  (if (== (`|GetArrayItem` (`self.Tags`)) _output)
    (`self.BajarPlaca`)
    (bind _outactors (`GameplayStatics.GetAllActorsOfClassWithTag` "/Game/SotanoFInal/BP_PuertaSotano.BP_PuertaSotano_C" "Puerta"))
    (bind _output_2 (`|GetArrayItem` _outactors))
    (if (== (`|GetArrayItem` (`Actor.Tags` _output_2)) _output)
      (`/Game/SotanoFInal/BP_PuertaSotano.AbrirPuerta` _output_2)
      (else
        (`/Game/SotanoFInal/BP_PuertaSotano.AbrirPuerta` (`|GetArrayItem` _outactors 1))))
    (else
      (`self.BajarPlaca`))))

(event `self.ReceiveActorEndOverlap`
  (params (OtherActor :type "Actor Object Reference"))
  ;[1 1 1] EndOverlp
  (`self.SubirPlaca`))

(event `SubirPlaca`
  (bind (_collisionlocation_x _collisionlocation_y _collisionlocation_z) (`KismetMathLibrary.BreakVector` (`self.CollisionLocation`)))
  (bind _returnvalue (- _collisionlocation_z 1.0))
  ;[1 1 1] SubirPlaca
  (`SceneComponent.K2_SetWorldLocation` (`self.Box`) (`KismetMathLibrary.MakeVector` _collisionlocation_x _collisionlocation_y _returnvalue) false false)
  (set `self.CollisionLocation` (`KismetMathLibrary.MakeVector` _collisionlocation_x _collisionlocation_y _returnvalue))
  (bind (_direction _movimiento) (`Timeline|Cronograma` :!via `PlayFromStart`)
    (:`Update`
      (bind _returnvalue_2 (`KismetMathLibrary.VLerp` (`self.CurrentLocation`) (`self.StartLocation`) _movimiento))
      (`SceneComponent.K2_SetWorldLocation` (`self.BasePlaca`) _returnvalue_2 false false)
      (set `self.CurrentLocation` _returnvalue_2))))

(event `BajarPlaca`
  (bind (_startlocation_x _startlocation_y _startlocation_z) (`KismetMathLibrary.BreakVector` (`self.StartLocation`)))
  ;[1 1 1] BajarPlaca
  (bind _output_get (set `self.EndLocation` (`KismetMathLibrary.MakeVector` _startlocation_x _startlocation_y (- _startlocation_z 5.0))))
  (bind (_direction _movimiento) (`Timeline|Cronograma_0` :!via `PlayFromStart`)
    (:`Update`
      (bind _returnvalue (`KismetMathLibrary.VLerp` (`self.CurrentLocation`) _output_get _movimiento))
      (`SceneComponent.K2_SetWorldLocation` (`self.BasePlaca`) _returnvalue false false)
      (set `self.CurrentLocation` _returnvalue))))

(fn `UserConstructionScript`)
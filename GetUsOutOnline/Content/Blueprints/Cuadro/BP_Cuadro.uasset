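; BP_Cuadro is a grabbable painting that swings open and enables collisions on the safe (BP_CajaFuerte).
; Each grab plays an opening sound; on alternate grabs, it rotates the scene component to a fixed yaw over time.
; The first opening goes through an RPC and multicast to enable the safe's collisions.
; Closing and timer-driven hand tracking (UpdateMovement) remain in unreachable code, so neither runs.
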(event `RPCHabilitar colisiones`
  (params (CajaFuerte :type "/Game/Blueprints/CajaFuerte/BP_CajaFuerte/BP_CajaFuerte Object Reference"))
  (`self.RPCHabilitarColisionesMulticast` CajaFuerte))

(event `RPCHabilitarColisionesMulticast`
  (params (CajaFuerte :type "/Game/Blueprints/CajaFuerte/BP_CajaFuerte/BP_CajaFuerte Object Reference"))
  (`/Game/Blueprints/CajaFuerte/BP_CajaFuerte/BP_CajaFuerte.HabilitarColisiones` CajaFuerte)
  (set `self.Habilitadas` true)
  (set `self.RotacionZ` 160.0 :!label _label)
  (`KismetSystemLibrary.MoveComponentTo` (`self.Scene`) (0.0 0.0 0.0) (`KismetMathLibrary.MakeRotator` 0.0 0.0 (`self.RotacionZ`)) false false 5.0))

(event `self.GrabComponent.OnDropped`
  (`KismetSystemLibrary.K2_ClearAndInvalidateTimerHandle` (`self.Timer`))
  (set `self.Motion Controller` null))

(event `self.GrabComponent.OnGrabbed`
  (params (`Motion Controller` :type "MotionControllerComponent Object Reference"))
  (`GameplayStatics.PlaySoundAtLocation` "/Game/Audio/Audio_PuertaAbriendose1Mitad.Audio_PuertaAbriendose1Mitad" (`self.K2_GetActorLocation`) (struct) 1.0 1.0 0.0 null null null null)
  (`/Engine/EditorBlueprintResources/StandardMacros.FlipFlop`
    (:`A`
      (if (`self.Habilitadas`)
        (goto _label)
        (else
          (bind _returnvalue (`GameplayStatics.GetActorOfClass` "/Game/Blueprints/CajaFuerte/BP_CajaFuerte/BP_CajaFuerte.BP_CajaFuerte_C"))
          (`self.RPCHabilitar colisiones` _returnvalue))))))

(fn `UpdateMovement`
  (locals (NewLocalVar :type "Float (double-precision)" :default 0.0))
  (bind _scene (`self.Scene`))
  (bind _grabcomponent (`self.GrabComponent`))
  (bind (_relativerotation_roll _relativerotation_pitch _relativerotation_yaw) (`KismetMathLibrary.BreakRotator` (`SceneComponent.RelativeRotation` _scene)))
  (bind _returnvalue_location (`KismetMathLibrary.BreakTransform` (`KismetMathLibrary.MakeRelativeTransform` (`SceneComponent.K2_GetComponentToWorld` (`self.Motion Controller`)) (`SceneComponent.K2_GetComponentToWorld` _grabcomponent))))
  (bind (_returnvalue_x _returnvalue_y) (`KismetMathLibrary.BreakVector` (- _returnvalue_location (`SceneComponent.RelativeLocation` _grabcomponent))))
  (`SceneComponent.K2_SetRelativeRotation` _scene (`KismetMathLibrary.MakeRotator` _relativerotation_roll _relativerotation_pitch (`KismetMathLibrary.FClamp` (+ _relativerotation_yaw _returnvalue_x _returnvalue_y) 1.0 160.0)) false false))

(fn `UserConstructionScript`)
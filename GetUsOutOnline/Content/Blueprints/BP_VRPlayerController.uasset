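; VR player controller Blueprint that carries a player number from the game instance into the controller in a networked game.
; On BeginPlay, instances without authority read NumJugador from BP_GameInstance and pass it through an RPC event, which stores it as PlayerNumber.
; A separate Numplayer function returns the player count from the lobby game mode, with debug prints for the result or a failed cast.
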(event `RPC_NumPlayer`
  (params (NewParam :type Integer))
  (set `self.PlayerNumber` NewParam)
  (`KismetSystemLibrary.PrintString` "NUMERO GUARDADO GAME INSTANCE" true true (struct :`G` 0.66 :`B` 1.0 :`A` 1.0) 10.0))

(event `self.ReceiveBeginPlay`
  (`/Engine/EditorBlueprintResources/ActorMacros.Switch Has Authority`
    (:`Remote`
      (bind _asbp_game_instance (cast `/Game/Blueprints/Lobby/Blueprint/BP_GameInstance` (`GameplayStatics.GetGameInstance`)))
      (`self.RPC_NumPlayer` (`/Game/Blueprints/Lobby/Blueprint/BP_GameInstance.NumJugador` _asbp_game_instance)))))

(fn `Numplayer`
  (returns (NumPlayers :type Integer))
  (bind _asbp_lobby_game_mode_base (cast `/Game/Blueprints/Lobby/Blueprint/BP_LobbyGameModeBase` (`GameplayStatics.GetGameMode`))
    (:`then`
      (bind _returnvalue (`GameModeBase.GetNumPlayers` _asbp_lobby_game_mode_base))
      (`KismetSystemLibrary.PrintString` (`KismetStringLibrary.Conv_IntToString` (`/Game/Blueprints/Lobby/Blueprint/BP_LobbyGameModeBase.NumPlayers` _asbp_lobby_game_mode_base)) true true (struct :`R` 1.0 :`G` 0.179633 :`A` 1.0) 50.0)
      (return _returnvalue))
    (:`CastFailed`
      (`KismetSystemLibrary.PrintString` "FALLA EL CASTRO" true true (struct :`G` 0.66 :`B` 1.0 :`A` 1.0) 500.0))))

(fn `UserConstructionScript`)
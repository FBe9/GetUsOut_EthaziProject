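; VR computer keypad puzzle with a four-digit code, then a two-digit triangles stage, each opening a BP_Mesilla_ordenador drawer.
; Overlap boxes animate buttons and, only without authority, send tagged digits, delete and OK through VRPawn, with a Pulsado debounce on digits.
; Multicast-named events update, reset and check the widget code, colouring it green or red.
; A separate event fills the post-it widget; several door and colour events are empty stubs.
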(event `self.Box_1.OnComponentEndOverlap`
  (params (OverlappedComponent :type "PrimitiveComponent Object Reference") (OtherActor :type "Actor Object Reference") (OtherComp :type "PrimitiveComponent Object Reference") (OtherBodyIndex :type Integer))
  (bind _v002_ordenador_botonesalcero_boton4 (`self.v002_Ordenador_BotonesAlCero_Boton4`))
  (bind (_relativelocation_x _relativelocation_y) (`KismetMathLibrary.BreakVector` (`SceneComponent.RelativeLocation` _v002_ordenador_botonesalcero_boton4)))
  ;[1 0.5511 0] Retorna a la posicion inical los botones cuando el objeto deja de estar encima
  (`KismetSystemLibrary.MoveComponentTo` _v002_ordenador_botonesalcero_boton4 (`KismetMathLibrary.MakeVector` _relativelocation_x _relativelocation_y 0.8) (struct) false false (`self.MovementSeconds`)))

(event `self.Box_4.OnComponentBeginOverlap`
  (params (OverlappedComponent :type "PrimitiveComponent Object Reference") (OtherActor :type "Actor Object Reference") (OtherComp :type "PrimitiveComponent Object Reference") (OtherBodyIndex :type Integer) (bFromSweep :type Boolean) (SweepResult :type "HitResult Structure (by ref)"))
  (bind _v002_ordenador_botonesalcero_boton7 (`self.v002_Ordenador_BotonesAlCero_Boton7`))
  (bind (_relativelocation_x _relativelocation_y _relativelocation_z) (`KismetMathLibrary.BreakVector` (`SceneComponent.RelativeLocation` _v002_ordenador_botonesalcero_boton7)))
  ;[1 0.5511 0] Cuando se pulse un botón lo mueve se llama al metodo ButtonAnimation pasandole el boton y el numero que tiene
  (if (not (`self.pulsado`))
    (set `self.pulsado` true)
    (`/Engine/EditorBlueprintResources/ActorMacros.Switch Has Authority`
      (:`Remote`
        (`KismetSystemLibrary.MoveComponentTo` _v002_ordenador_botonesalcero_boton7 (`KismetMathLibrary.MakeVector` _relativelocation_x _relativelocation_y (`KismetMathLibrary.FClamp` (- _relativelocation_z 0.2) 0.0 0.8)) (struct) false false (`self.MovementSeconds`))
        (`self.ButtonAnimation` null (`KismetStringLibrary.Conv_StringToInt` (`KismetStringLibrary.Conv_NameToString` (`|GetArrayItem` (`ActorComponent.ComponentTags` OverlappedComponent)))))
        ;[1 0.5511 0] Retorna a la posicion inical los botones cuando el objeto deja de estar encima
        (`KismetSystemLibrary.Delay` 3.0 :!label _label)
        (set `self.pulsado` false)))))

(event `self.Box_9.OnComponentEndOverlap`
  (params (OverlappedComponent :type "PrimitiveComponent Object Reference") (OtherActor :type "Actor Object Reference") (OtherComp :type "PrimitiveComponent Object Reference") (OtherBodyIndex :type Integer))
  (bind _v002_ordenador_botonesalcero_boton8 (`self.v002_Ordenador_BotonesAlCero_Boton8`))
  (bind (_relativelocation_x _relativelocation_y) (`KismetMathLibrary.BreakVector` (`SceneComponent.RelativeLocation` _v002_ordenador_botonesalcero_boton8)))
  ;[1 0.5511 0] Retorna a la posicion inical los botones cuando el objeto deja de estar encima
  (set `self.pulsado` false)
  (`KismetSystemLibrary.MoveComponentTo` _v002_ordenador_botonesalcero_boton8 (`KismetMathLibrary.MakeVector` _relativelocation_x _relativelocation_y 0.8) (struct) false false (`self.MovementSeconds`)))

(event `self.Box_9.OnComponentBeginOverlap`
  (params (OverlappedComponent :type "PrimitiveComponent Object Reference") (OtherActor :type "Actor Object Reference") (OtherComp :type "PrimitiveComponent Object Reference") (OtherBodyIndex :type Integer) (bFromSweep :type Boolean) (SweepResult :type "HitResult Structure (by ref)"))
  (bind _v002_ordenador_botonesalcero_boton8 (`self.v002_Ordenador_BotonesAlCero_Boton8`))
  (bind (_relativelocation_x _relativelocation_y _relativelocation_z) (`KismetMathLibrary.BreakVector` (`SceneComponent.RelativeLocation` _v002_ordenador_botonesalcero_boton8)))
  ;[1 0.5511 0] Cuando se pulse un botón lo mueve se llama al metodo ButtonAnimation pasandole el boton y el numero que tiene
  (if (not (`self.pulsado`))
    (set `self.pulsado` true)
    (`/Engine/EditorBlueprintResources/ActorMacros.Switch Has Authority`
      (:`Remote`
        (`KismetSystemLibrary.MoveComponentTo` _v002_ordenador_botonesalcero_boton8 (`KismetMathLibrary.MakeVector` _relativelocation_x _relativelocation_y (`KismetMathLibrary.FClamp` (- _relativelocation_z 0.2) 0.0 0.8)) (struct) false false (`self.MovementSeconds`))
        (`self.ButtonAnimation` null (`KismetStringLibrary.Conv_StringToInt` (`KismetStringLibrary.Conv_NameToString` (`|GetArrayItem` (`ActorComponent.ComponentTags` OverlappedComponent)))))
        (`KismetSystemLibrary.Delay` 3.0 :!label _label_2)
        (set `self.pulsado` false)))))

(event `self.Box_8.OnComponentEndOverlap`
  (params (OverlappedComponent :type "PrimitiveComponent Object Reference") (OtherActor :type "Actor Object Reference") (OtherComp :type "PrimitiveComponent Object Reference") (OtherBodyIndex :type Integer))
  (bind _v002_ordenador_botonesalcero_boton9 (`self.v002_Ordenador_BotonesAlCero_Boton9`))
  (bind (_relativelocation_x _relativelocation_y) (`KismetMathLibrary.BreakVector` (`SceneComponent.RelativeLocation` _v002_ordenador_botonesalcero_boton9)))
  ;[1 0.5511 0] Retorna a la posicion inical los botones cuando el objeto deja de estar encima
  (set `self.pulsado` false)
  (`KismetSystemLibrary.MoveComponentTo` _v002_ordenador_botonesalcero_boton9 (`KismetMathLibrary.MakeVector` _relativelocation_x _relativelocation_y 0.8) (struct) false false (`self.MovementSeconds`)))

(event `self.Box_8.OnComponentBeginOverlap`
  (params (OverlappedComponent :type "PrimitiveComponent Object Reference") (OtherActor :type "Actor Object Reference") (OtherComp :type "PrimitiveComponent Object Reference") (OtherBodyIndex :type Integer) (bFromSweep :type Boolean) (SweepResult :type "HitResult Structure (by ref)"))
  (bind _v002_ordenador_botonesalcero_boton9 (`self.v002_Ordenador_BotonesAlCero_Boton9`))
  (bind (_relativelocation_x _relativelocation_y _relativelocation_z) (`KismetMathLibrary.BreakVector` (`SceneComponent.RelativeLocation` _v002_ordenador_botonesalcero_boton9)))
  ;[1 0.5511 0] Cuando se pulse un botón lo mueve se llama al metodo ButtonAnimation pasandole el boton y el numero que tiene
  (if (not (`self.pulsado`))
    (set `self.pulsado` true)
    (`/Engine/EditorBlueprintResources/ActorMacros.Switch Has Authority`
      (:`Remote`
        (`KismetSystemLibrary.MoveComponentTo` _v002_ordenador_botonesalcero_boton9 (`KismetMathLibrary.MakeVector` _relativelocation_x _relativelocation_y (`KismetMathLibrary.FClamp` (- _relativelocation_z 0.2) 0.0 0.8)) (struct) false false (`self.MovementSeconds`))
        (`self.ButtonAnimation` null (`KismetStringLibrary.Conv_StringToInt` (`KismetStringLibrary.Conv_NameToString` (`|GetArrayItem` (`ActorComponent.ComponentTags` OverlappedComponent)))))
        (goto _label_2)))))

(event `self.Box_0.OnComponentEndOverlap`
  (params (OverlappedComponent :type "PrimitiveComponent Object Reference") (OtherActor :type "Actor Object Reference") (OtherComp :type "PrimitiveComponent Object Reference") (OtherBodyIndex :type Integer))
  (bind _v002_ordenador_botonesalcero_boton11 (`self.v002_Ordenador_BotonesAlCero_Boton11`))
  (bind (_relativelocation_x _relativelocation_y) (`KismetMathLibrary.BreakVector` (`SceneComponent.RelativeLocation` _v002_ordenador_botonesalcero_boton11)))
  ;[1 0.5511 0] Retorna a la posicion inical los botones cuando el objeto deja de estar encima
  (`KismetSystemLibrary.MoveComponentTo` _v002_ordenador_botonesalcero_boton11 (`KismetMathLibrary.MakeVector` _relativelocation_x _relativelocation_y 0.8) (struct) false false (`self.MovementSeconds`)))

(event `self.Box_3.OnComponentBeginOverlap`
  (params (OverlappedComponent :type "PrimitiveComponent Object Reference") (OtherActor :type "Actor Object Reference") (OtherComp :type "PrimitiveComponent Object Reference") (OtherBodyIndex :type Integer) (bFromSweep :type Boolean) (SweepResult :type "HitResult Structure (by ref)"))
  (bind _v002_ordenador_botonesalcero_boton2 (`self.v002_Ordenador_BotonesAlCero_Boton2`))
  (bind (_relativelocation_x _relativelocation_y _relativelocation_z) (`KismetMathLibrary.BreakVector` (`SceneComponent.RelativeLocation` _v002_ordenador_botonesalcero_boton2)))
  ;[1 0.5511 0] Cuando se pulse un botón lo mueve se llama al metodo ButtonAnimation pasandole el boton y el numero que tiene
  (if (not (`self.pulsado`))
    (set `self.pulsado` true)
    (`/Engine/EditorBlueprintResources/ActorMacros.Switch Has Authority`
      (:`Remote`
        (`KismetSystemLibrary.MoveComponentTo` _v002_ordenador_botonesalcero_boton2 (`KismetMathLibrary.MakeVector` _relativelocation_x _relativelocation_y (`KismetMathLibrary.FClamp` (- _relativelocation_z 0.2) 0.0 0.8)) (struct) false false (`self.MovementSeconds`))
        (`self.ButtonAnimation` null (`KismetStringLibrary.Conv_StringToInt` (`KismetStringLibrary.Conv_NameToString` (`|GetArrayItem` (`ActorComponent.ComponentTags` OverlappedComponent)))))
        (goto _label)))))

(event `ButtonReturnPosition`
  (params (Button :type "StaticMeshComponent Object Reference") (Box :type "BoxComponent Object Reference") (BoxOverlap :type Boolean))
  ;[1 0.5511 0] Retorna a la posicion inical los botones cuando el objeto deja de estar encima
)

(event `self.Box_7.OnComponentEndOverlap`
  (params (OverlappedComponent :type "PrimitiveComponent Object Reference") (OtherActor :type "Actor Object Reference") (OtherComp :type "PrimitiveComponent Object Reference") (OtherBodyIndex :type Integer))
  (bind _v002_ordenador_botonesalcero_boton10 (`self.v002_Ordenador_BotonesAlCero_Boton10`))
  (bind (_relativelocation_x _relativelocation_y) (`KismetMathLibrary.BreakVector` (`SceneComponent.RelativeLocation` _v002_ordenador_botonesalcero_boton10)))
  ;[1 0.5511 0] Retorna a la posicion inical los botones cuando el objeto deja de estar encima
  (set `self.pulsado` false)
  (`KismetSystemLibrary.MoveComponentTo` _v002_ordenador_botonesalcero_boton10 (`KismetMathLibrary.MakeVector` _relativelocation_x _relativelocation_y 0.8) (struct) false false (`self.MovementSeconds`)))

(event `self.Box_2.OnComponentBeginOverlap`
  (params (OverlappedComponent :type "PrimitiveComponent Object Reference") (OtherActor :type "Actor Object Reference") (OtherComp :type "PrimitiveComponent Object Reference") (OtherBodyIndex :type Integer) (bFromSweep :type Boolean) (SweepResult :type "HitResult Structure (by ref)"))
  (bind _v002_ordenador_botonesalcero_boton3 (`self.v002_Ordenador_BotonesAlCero_Boton3`))
  (bind (_relativelocation_x _relativelocation_y _relativelocation_z) (`KismetMathLibrary.BreakVector` (`SceneComponent.RelativeLocation` _v002_ordenador_botonesalcero_boton3)))
  ;[1 0.5511 0] Cuando se pulse un botón lo mueve se llama al metodo ButtonAnimation pasandole el boton y el numero que tiene
  (if (not (`self.pulsado`))
    (set `self.pulsado` true)
    (`/Engine/EditorBlueprintResources/ActorMacros.Switch Has Authority`
      (:`Remote`
        (`KismetSystemLibrary.MoveComponentTo` _v002_ordenador_botonesalcero_boton3 (`KismetMathLibrary.MakeVector` _relativelocation_x _relativelocation_y (`KismetMathLibrary.FClamp` (- _relativelocation_z 0.2) 0.0 0.8)) (struct) false false (`self.MovementSeconds`))
        (`self.ButtonAnimation` null (`KismetStringLibrary.Conv_StringToInt` (`KismetStringLibrary.Conv_NameToString` (`|GetArrayItem` (`ActorComponent.ComponentTags` OverlappedComponent)))))
        (goto _label)))))

(event `self.Box_ok.OnComponentEndOverlap`
  (params (OverlappedComponent :type "PrimitiveComponent Object Reference") (OtherActor :type "Actor Object Reference") (OtherComp :type "PrimitiveComponent Object Reference") (OtherBodyIndex :type Integer))
  (bind _v002_ordenador_botonesalcero_boton1 (`self.v002_Ordenador_BotonesAlCero_Boton1`))
  (bind (_relativelocation_x _relativelocation_y) (`KismetMathLibrary.BreakVector` (`SceneComponent.RelativeLocation` _v002_ordenador_botonesalcero_boton1)))
  ;[1 0.5511 0] Retorna a la posicion inical los botones cuando el objeto deja de estar encima
  (`KismetSystemLibrary.MoveComponentTo` _v002_ordenador_botonesalcero_boton1 (`KismetMathLibrary.MakeVector` _relativelocation_x _relativelocation_y 0.8) (struct) false false (`self.MovementSeconds`)))

(event `self.Box_7.OnComponentBeginOverlap`
  (params (OverlappedComponent :type "PrimitiveComponent Object Reference") (OtherActor :type "Actor Object Reference") (OtherComp :type "PrimitiveComponent Object Reference") (OtherBodyIndex :type Integer) (bFromSweep :type Boolean) (SweepResult :type "HitResult Structure (by ref)"))
  (bind _v002_ordenador_botonesalcero_boton10 (`self.v002_Ordenador_BotonesAlCero_Boton10`))
  (bind (_relativelocation_x _relativelocation_y _relativelocation_z) (`KismetMathLibrary.BreakVector` (`SceneComponent.RelativeLocation` _v002_ordenador_botonesalcero_boton10)))
  ;[1 0.5511 0] Cuando se pulse un botón lo mueve se llama al metodo ButtonAnimation pasandole el boton y el numero que tiene
  (if (not (`self.pulsado`))
    (set `self.pulsado` true)
    (`/Engine/EditorBlueprintResources/ActorMacros.Switch Has Authority`
      (:`Remote`
        (`KismetSystemLibrary.MoveComponentTo` _v002_ordenador_botonesalcero_boton10 (`KismetMathLibrary.MakeVector` _relativelocation_x _relativelocation_y (`KismetMathLibrary.FClamp` (- _relativelocation_z 0.2) 0.0 0.8)))
        (`self.ButtonAnimation` null (`KismetStringLibrary.Conv_StringToInt` (`KismetStringLibrary.Conv_NameToString` (`|GetArrayItem` (`ActorComponent.ComponentTags` OverlappedComponent)))))
        (goto _label_2)))))

(event `self.Box_6.OnComponentEndOverlap`
  (params (OverlappedComponent :type "PrimitiveComponent Object Reference") (OtherActor :type "Actor Object Reference") (OtherComp :type "PrimitiveComponent Object Reference") (OtherBodyIndex :type Integer))
  (bind _v002_ordenador_botonesalcero_boton5 (`self.v002_Ordenador_BotonesAlCero_Boton5`))
  (bind (_relativelocation_x _relativelocation_y) (`KismetMathLibrary.BreakVector` (`SceneComponent.RelativeLocation` _v002_ordenador_botonesalcero_boton5)))
  ;[1 0.5511 0] Retorna a la posicion inical los botones cuando el objeto deja de estar encima
  (`KismetSystemLibrary.MoveComponentTo` _v002_ordenador_botonesalcero_boton5 (`KismetMathLibrary.MakeVector` _relativelocation_x _relativelocation_y 0.8) (struct) false false (`self.MovementSeconds`)))

(event `self.Box_delete.OnComponentEndOverlap`
  (params (OverlappedComponent :type "PrimitiveComponent Object Reference") (OtherActor :type "Actor Object Reference") (OtherComp :type "PrimitiveComponent Object Reference") (OtherBodyIndex :type Integer))
  (bind _v002_ordenador_botonesalcero_boton12 (`self.v002_Ordenador_BotonesAlCero_Boton12`))
  (bind (_relativelocation_x _relativelocation_y) (`KismetMathLibrary.BreakVector` (`SceneComponent.RelativeLocation` _v002_ordenador_botonesalcero_boton12)))
  ;[1 0.5511 0] Retorna a la posicion inical los botones cuando el objeto deja de estar encima
  (`KismetSystemLibrary.MoveComponentTo` _v002_ordenador_botonesalcero_boton12 (`KismetMathLibrary.MakeVector` _relativelocation_x _relativelocation_y 0.8) (struct) false false (`self.MovementSeconds`)))

(event `self.Box_1.OnComponentBeginOverlap`
  (params (OverlappedComponent :type "PrimitiveComponent Object Reference") (OtherActor :type "Actor Object Reference") (OtherComp :type "PrimitiveComponent Object Reference") (OtherBodyIndex :type Integer) (bFromSweep :type Boolean) (SweepResult :type "HitResult Structure (by ref)"))
  (bind _v002_ordenador_botonesalcero_boton4 (`self.v002_Ordenador_BotonesAlCero_Boton4`))
  (bind (_relativelocation_x _relativelocation_y _relativelocation_z) (`KismetMathLibrary.BreakVector` (`SceneComponent.RelativeLocation` _v002_ordenador_botonesalcero_boton4)))
  ;[1 0.5511 0] Cuando se pulse un botón lo mueve se llama al metodo ButtonAnimation pasandole el boton y el numero que tiene
  (if (not (`self.pulsado`))
    (set `self.pulsado` true)
    (`/Engine/EditorBlueprintResources/ActorMacros.Switch Has Authority`
      (:`Remote`
        (`KismetSystemLibrary.MoveComponentTo` _v002_ordenador_botonesalcero_boton4 (`KismetMathLibrary.MakeVector` _relativelocation_x _relativelocation_y (`KismetMathLibrary.FClamp` (- _relativelocation_z 0.2) 0.0 0.8)) (struct) false false (`self.MovementSeconds`))
        (`self.ButtonAnimation` null (`KismetStringLibrary.Conv_StringToInt` (`KismetStringLibrary.Conv_NameToString` (`|GetArrayItem` (`ActorComponent.ComponentTags` OverlappedComponent)))))
        (goto _label)))))

(event `self.Box_6.OnComponentBeginOverlap`
  (params (OverlappedComponent :type "PrimitiveComponent Object Reference") (OtherActor :type "Actor Object Reference") (OtherComp :type "PrimitiveComponent Object Reference") (OtherBodyIndex :type Integer) (bFromSweep :type Boolean) (SweepResult :type "HitResult Structure (by ref)"))
  (bind _v002_ordenador_botonesalcero_boton5 (`self.v002_Ordenador_BotonesAlCero_Boton5`))
  (bind (_relativelocation_x _relativelocation_y _relativelocation_z) (`KismetMathLibrary.BreakVector` (`SceneComponent.RelativeLocation` _v002_ordenador_botonesalcero_boton5)))
  ;[1 0.5511 0] Cuando se pulse un botón lo mueve se llama al metodo ButtonAnimation pasandole el boton y el numero que tiene
  (if (not (`self.pulsado`))
    (set `self.pulsado` true)
    (`/Engine/EditorBlueprintResources/ActorMacros.Switch Has Authority`
      (:`Remote`
        (`KismetSystemLibrary.MoveComponentTo` _v002_ordenador_botonesalcero_boton5 (`KismetMathLibrary.MakeVector` _relativelocation_x _relativelocation_y (`KismetMathLibrary.FClamp` (- _relativelocation_z 0.2) 0.0 0.8)) (struct) false false (`self.MovementSeconds`))
        (`self.ButtonAnimation` null (`KismetStringLibrary.Conv_StringToInt` (`KismetStringLibrary.Conv_NameToString` (`|GetArrayItem` (`ActorComponent.ComponentTags` OverlappedComponent)))))
        (goto _label_2)))))

(event `self.Box_5.OnComponentEndOverlap`
  (params (OverlappedComponent :type "PrimitiveComponent Object Reference") (OtherActor :type "Actor Object Reference") (OtherComp :type "PrimitiveComponent Object Reference") (OtherBodyIndex :type Integer))
  (bind _v002_ordenador_botonesalcero_boton6 (`self.v002_Ordenador_BotonesAlCero_Boton6`))
  (bind (_relativelocation_x _relativelocation_y) (`KismetMathLibrary.BreakVector` (`SceneComponent.RelativeLocation` _v002_ordenador_botonesalcero_boton6)))
  ;[1 0.5511 0] Retorna a la posicion inical los botones cuando el objeto deja de estar encima
  (`KismetSystemLibrary.MoveComponentTo` _v002_ordenador_botonesalcero_boton6 (`KismetMathLibrary.MakeVector` _relativelocation_x _relativelocation_y 0.8)))

(event `self.Box_3.OnComponentEndOverlap`
  (params (OverlappedComponent :type "PrimitiveComponent Object Reference") (OtherActor :type "Actor Object Reference") (OtherComp :type "PrimitiveComponent Object Reference") (OtherBodyIndex :type Integer))
  (bind _v002_ordenador_botonesalcero_boton2 (`self.v002_Ordenador_BotonesAlCero_Boton2`))
  (bind (_relativelocation_x _relativelocation_y) (`KismetMathLibrary.BreakVector` (`SceneComponent.RelativeLocation` _v002_ordenador_botonesalcero_boton2)))
  ;[1 0.5511 0] Retorna a la posicion inical los botones cuando el objeto deja de estar encima
  (`KismetSystemLibrary.MoveComponentTo` _v002_ordenador_botonesalcero_boton2 (`KismetMathLibrary.MakeVector` _relativelocation_x _relativelocation_y 0.8) (struct) false false (`self.MovementSeconds`)))

(event `self.Box_0.OnComponentBeginOverlap`
  (params (OverlappedComponent :type "PrimitiveComponent Object Reference") (OtherActor :type "Actor Object Reference") (OtherComp :type "PrimitiveComponent Object Reference") (OtherBodyIndex :type Integer) (bFromSweep :type Boolean) (SweepResult :type "HitResult Structure (by ref)"))
  (bind _v002_ordenador_botonesalcero_boton11 (`self.v002_Ordenador_BotonesAlCero_Boton11`))
  (bind (_relativelocation_x _relativelocation_y _relativelocation_z) (`KismetMathLibrary.BreakVector` (`SceneComponent.RelativeLocation` _v002_ordenador_botonesalcero_boton11)))
  ;[1 0.5511 0] Cuando se pulse un botón lo mueve se llama al metodo ButtonAnimation pasandole el boton y el numero que tiene
  (if (not (`self.pulsado`))
    (set `self.pulsado` true)
    (`/Engine/EditorBlueprintResources/ActorMacros.Switch Has Authority`
      (:`Remote`
        (`KismetSystemLibrary.MoveComponentTo` _v002_ordenador_botonesalcero_boton11 (`KismetMathLibrary.MakeVector` _relativelocation_x _relativelocation_y (`KismetMathLibrary.FClamp` (- _relativelocation_z 0.2) 0.0 0.8)) (struct) false false (`self.MovementSeconds`))
        (`self.ButtonAnimation` null (`KismetStringLibrary.Conv_StringToInt` (`KismetStringLibrary.Conv_NameToString` (`|GetArrayItem` (`ActorComponent.ComponentTags` OverlappedComponent)))))
        (goto _label)))))

(event `self.Box_5.OnComponentBeginOverlap`
  (params (OverlappedComponent :type "PrimitiveComponent Object Reference") (OtherActor :type "Actor Object Reference") (OtherComp :type "PrimitiveComponent Object Reference") (OtherBodyIndex :type Integer) (bFromSweep :type Boolean) (SweepResult :type "HitResult Structure (by ref)"))
  (bind _v002_ordenador_botonesalcero_boton6 (`self.v002_Ordenador_BotonesAlCero_Boton6`))
  (bind (_relativelocation_x _relativelocation_y _relativelocation_z) (`KismetMathLibrary.BreakVector` (`SceneComponent.RelativeLocation` _v002_ordenador_botonesalcero_boton6)))
  ;[1 0.5511 0] Cuando se pulse un botón lo mueve se llama al metodo ButtonAnimation pasandole el boton y el numero que tiene
  (if (not (`self.pulsado`))
    (set `self.pulsado` true)
    (`/Engine/EditorBlueprintResources/ActorMacros.Switch Has Authority`
      (:`Remote`
        (`KismetSystemLibrary.MoveComponentTo` _v002_ordenador_botonesalcero_boton6 (`KismetMathLibrary.MakeVector` _relativelocation_x _relativelocation_y (`KismetMathLibrary.FClamp` (- _relativelocation_z 0.2) 0.0 0.8)) (struct) false false (`self.MovementSeconds`))
        (`self.ButtonAnimation` null (`KismetStringLibrary.Conv_StringToInt` (`KismetStringLibrary.Conv_NameToString` (`|GetArrayItem` (`ActorComponent.ComponentTags` OverlappedComponent)))))
        (goto _label_2)))))

(event `self.Box_4.OnComponentEndOverlap`
  (params (OverlappedComponent :type "PrimitiveComponent Object Reference") (OtherActor :type "Actor Object Reference") (OtherComp :type "PrimitiveComponent Object Reference") (OtherBodyIndex :type Integer))
  (bind _v002_ordenador_botonesalcero_boton7 (`self.v002_Ordenador_BotonesAlCero_Boton7`))
  (bind (_relativelocation_x _relativelocation_y) (`KismetMathLibrary.BreakVector` (`SceneComponent.RelativeLocation` _v002_ordenador_botonesalcero_boton7)))
  ;[1 0.5511 0] Retorna a la posicion inical los botones cuando el objeto deja de estar encima
  (`KismetSystemLibrary.MoveComponentTo` _v002_ordenador_botonesalcero_boton7 (`KismetMathLibrary.MakeVector` _relativelocation_x _relativelocation_y 0.8)))

(event `self.Box_2.OnComponentEndOverlap`
  (params (OverlappedComponent :type "PrimitiveComponent Object Reference") (OtherActor :type "Actor Object Reference") (OtherComp :type "PrimitiveComponent Object Reference") (OtherBodyIndex :type Integer))
  (bind _v002_ordenador_botonesalcero_boton3 (`self.v002_Ordenador_BotonesAlCero_Boton3`))
  (bind (_relativelocation_x _relativelocation_y) (`KismetMathLibrary.BreakVector` (`SceneComponent.RelativeLocation` _v002_ordenador_botonesalcero_boton3)))
  ;[1 0.5511 0] Retorna a la posicion inical los botones cuando el objeto deja de estar encima
  (`KismetSystemLibrary.MoveComponentTo` _v002_ordenador_botonesalcero_boton3 (`KismetMathLibrary.MakeVector` _relativelocation_x _relativelocation_y 0.8) (struct) false false (`self.MovementSeconds`)))

(event `self.Box_ok.OnComponentBeginOverlap`
  (params (OverlappedComponent :type "PrimitiveComponent Object Reference") (OtherActor :type "Actor Object Reference") (OtherComp :type "PrimitiveComponent Object Reference") (OtherBodyIndex :type Integer) (bFromSweep :type Boolean) (SweepResult :type "HitResult Structure (by ref)"))
  (bind _v002_ordenador_botonesalcero_boton1 (`self.v002_Ordenador_BotonesAlCero_Boton1`))
  (bind (_relativelocation_x _relativelocation_y _relativelocation_z) (`KismetMathLibrary.BreakVector` (`SceneComponent.RelativeLocation` _v002_ordenador_botonesalcero_boton1)))
  ;[1 0.5342 0] Cuando se pulsa el boton ok(la colision) mueve el boton hacia atras y llama al evento CheckCorrectCode del WID_PantallaCajaFuerte
  (`/Engine/EditorBlueprintResources/ActorMacros.Switch Has Authority`
    (:`Remote`
      (`KismetSystemLibrary.MoveComponentTo` _v002_ordenador_botonesalcero_boton1 (`KismetMathLibrary.MakeVector` _relativelocation_x _relativelocation_y (`KismetMathLibrary.FClamp` (- _relativelocation_z 0.2) 0.0 0.8)) (struct) false false (`self.MovementSeconds`))
      (if (not (`self.Open?`))
        (bind _asvrpawn (cast `/Game/VRTemplate/Blueprints/VRPawn` (`GameplayStatics.GetPlayerCharacter` 0)))
        (`/Game/VRTemplate/Blueprints/VRPawn.OKOrdenador` _asvrpawn self)))))

(event `ChangeValu`
  (params (Numero :type Integer))
  (bind _contador (`self.Contador`))
  ;[1 0.2217 0.09193] Mueve el boton correspondiente y llama al metodo ChangeValue del WID_PantallaCajaFuerte
  (`self.ChangeValueMulticast` Numero _contador)
  (if (`self.segundoNivel`)
    (if (not (== _contador 2))
      (`/Engine/EditorBlueprintResources/StandardMacros.IncrementInt` _contador :!label _label_3))
    (elif (not (== _contador 4))
      (goto _label_3))))

(event `ButtonAnimation`
  (params (BotonPresionado :type "StaticMeshComponent Object Reference") (Numero :type Integer))
  ;[1 0.2217 0.09193] Mueve el boton correspondiente y llama al metodo ChangeValue del WID_PantallaCajaFuerte
  (bind _asvrpawn (cast `/Game/VRTemplate/Blueprints/VRPawn` (`GameplayStatics.GetPlayerCharacter` 0)))
  (`/Game/VRTemplate/Blueprints/VRPawn.ChangeValue` _asvrpawn self Numero))

(event `self.Box_delete.OnComponentBeginOverlap`
  (params (OverlappedComponent :type "PrimitiveComponent Object Reference") (OtherActor :type "Actor Object Reference") (OtherComp :type "PrimitiveComponent Object Reference") (OtherBodyIndex :type Integer) (bFromSweep :type Boolean) (SweepResult :type "HitResult Structure (by ref)"))
  (bind _contador (`self.Contador`))
  (bind _v002_ordenador_botonesalcero_boton12 (`self.v002_Ordenador_BotonesAlCero_Boton12`))
  (bind (_relativelocation_x _relativelocation_y _relativelocation_z) (`KismetMathLibrary.BreakVector` (`SceneComponent.RelativeLocation` _v002_ordenador_botonesalcero_boton12)))
  ;[1 0.5342 0] Cuando se pulsa el boton delete(la colision) mueve el boton hacia atras y llama al evento Reset del WID_PantallaCajaFuerte
  (`/Engine/EditorBlueprintResources/ActorMacros.Switch Has Authority`
    (:`Remote`
      (`KismetSystemLibrary.MoveComponentTo` _v002_ordenador_botonesalcero_boton12 (`KismetMathLibrary.MakeVector` _relativelocation_x _relativelocation_y (`KismetMathLibrary.FClamp` (- _relativelocation_z 0.2) 0.0 0.8)) (struct) false false (`self.MovementSeconds`))
      (if (not (== _contador 0))
        (bind _asvrpawn (cast `/Game/VRTemplate/Blueprints/VRPawn` (`GameplayStatics.GetPlayerCharacter` 0)))
        (`/Game/VRTemplate/Blueprints/VRPawn.ResetNormalOrdenador` _asvrpawn self _contador)))))

(event `SetOpen`
  ;[1 0.1885 0.219] Pone la variable Open? en true y añade un sonido al boton
  (set `self.Open?` true)
  (`GameplayStatics.PlaySound2D` "/Engine/EngineSounds/1kSineTonePing.1kSineTonePing" 1.0 1.0 0.0 null null))

(event `OpenDoor`
  ;[1 0.212 0.202] Abre la puerta, cambia el material de la pantalla por uno verde y  hace sonar un sonido
)

(event `ResetColor`
  ;[1 0.1885 0.219] Resetea el color del marco y setea el contador a 0
)

(event `PostitContraseña`
  (params (Players :type Integer))
  (bind _aswid_post_it (cast `/Game/Widgets/WidgetsOrdenador/WID_PostIt` (`WidgetComponent.GetWidget` (`self.PostIt`))))
  (`/Game/Widgets/WidgetsOrdenador/WID_PostIt.ChangeValue` _aswid_post_it Players))

(event `SetErrorColor`
  ;[1 0.2135 0.2392] Pone color rojo cuando se introduce un codigo incorrecto
)

(event `ChangeValue`
  (params (Num :type Integer) (Position :type Integer))
  ;[1 1 1] Muestra el numero introducido en el txt correspondiente
  (`self.ChangeValueMulticast` Num Position))

(event `SetCode`
  ;[1 1 1] Guarda el codigo actual en una variable
  (if (`self.segundoNivel`)
    (bind _aswid_pantalla_ordenador_triangulos (cast `/Game/Widgets/WidgetsOrdenador/WID_PantallaOrdenadorTriangulos` (`WidgetComponent.GetWidget` (`self.Triangulos`))))
    (set `/Game/Widgets/WidgetsOrdenador/WID_PantallaOrdenadorTriangulos.CodigoIntroducido` (`KismetStringLibrary.Concat_StrStr` (`KismetTextLibrary.Conv_TextToString` (`TextBlock.Text` (`/Game/Widgets/WidgetsOrdenador/WID_PantallaOrdenadorTriangulos.PWD_1` _aswid_pantalla_ordenador_triangulos))) (`KismetTextLibrary.Conv_TextToString` (`TextBlock.Text` (`/Game/Widgets/WidgetsOrdenador/WID_PantallaOrdenadorTriangulos.PWD_2` _aswid_pantalla_ordenador_triangulos)))) _aswid_pantalla_ordenador_triangulos)
    (else
      (bind _aswid_pantalla_ordenador (cast `/Game/Widgets/WidgetsOrdenador/WID_PantallaOrdenador` (`WidgetComponent.GetWidget` (`self.Widget`))))
      (set `/Game/Widgets/WidgetsOrdenador/WID_PantallaOrdenador.CodigoIntroducido` (`KismetStringLibrary.Concat_StrStr` (`KismetTextLibrary.Conv_TextToString` (`TextBlock.Text` (`/Game/Widgets/WidgetsOrdenador/WID_PantallaOrdenador.PWD_1` _aswid_pantalla_ordenador))) (`KismetTextLibrary.Conv_TextToString` (`TextBlock.Text` (`/Game/Widgets/WidgetsOrdenador/WID_PantallaOrdenador.PWD_2` _aswid_pantalla_ordenador))) (`KismetTextLibrary.Conv_TextToString` (`TextBlock.Text` (`/Game/Widgets/WidgetsOrdenador/WID_PantallaOrdenador.PWD_3` _aswid_pantalla_ordenador))) (`KismetTextLibrary.Conv_TextToString` (`TextBlock.Text` (`/Game/Widgets/WidgetsOrdenador/WID_PantallaOrdenador.PWD_4` _aswid_pantalla_ordenador)))) _aswid_pantalla_ordenador))))

(event `ChangeValueMulticast`
  (params (Num :type Integer) (Position :type Integer))
  ;[1 1 1] Muestra el numero introducido en el txt correspondiente
  (if (`self.segundoNivel`)
    (bind _aswid_pantalla_ordenador_triangulos (cast `/Game/Widgets/WidgetsOrdenador/WID_PantallaOrdenadorTriangulos` (`WidgetComponent.GetWidget` (`self.Triangulos`))))
    (switch `int` Position
      (:`0`
        (`TextBlock.SetText` (`/Game/Widgets/WidgetsOrdenador/WID_PantallaOrdenadorTriangulos.PWD_1` _aswid_pantalla_ordenador_triangulos) (`KismetTextLibrary.Conv_IntToText` Num)))
      (:`1`
        (`TextBlock.SetText` (`/Game/Widgets/WidgetsOrdenador/WID_PantallaOrdenadorTriangulos.PWD_2` _aswid_pantalla_ordenador_triangulos) (`KismetTextLibrary.Conv_IntToText` Num))))
    (else
      (bind _aswid_pantalla_ordenador (cast `/Game/Widgets/WidgetsOrdenador/WID_PantallaOrdenador` (`WidgetComponent.GetWidget` (`self.Widget`))))
      (switch `int` Position
        (:`0`
          (`TextBlock.SetText` (`/Game/Widgets/WidgetsOrdenador/WID_PantallaOrdenador.PWD_1` _aswid_pantalla_ordenador) (`KismetTextLibrary.Conv_IntToText` Num)))
        (:`1`
          (`TextBlock.SetText` (`/Game/Widgets/WidgetsOrdenador/WID_PantallaOrdenador.PWD_2` _aswid_pantalla_ordenador) (`KismetTextLibrary.Conv_IntToText` Num)))
        (:`2`
          (`TextBlock.SetText` (`/Game/Widgets/WidgetsOrdenador/WID_PantallaOrdenador.PWD_3` _aswid_pantalla_ordenador) (`KismetTextLibrary.Conv_IntToText` Num)))
        (:`3`
          (`TextBlock.SetText` (`/Game/Widgets/WidgetsOrdenador/WID_PantallaOrdenador.PWD_4` _aswid_pantalla_ordenador) (`KismetTextLibrary.Conv_IntToText` Num))))))
  (`self.SetCode`))

(event `CheckCorrectCode`
  ;[1 1 1] Comprueba si el código introducido es correcto
  (`self.CheckCorrectCodeMulticast`))

(event `CheckCorrectCodeMulticast`
  ;[1 1 1] Comprueba si el código introducido es correcto
  (bind _aswid_pantalla_ordenador (cast `/Game/Widgets/WidgetsOrdenador/WID_PantallaOrdenador` (`WidgetComponent.GetWidget` (`self.Widget`))))
  (if (`self.segundoNivel`)
    (bind _aswid_pantalla_ordenador_triangulos (cast `/Game/Widgets/WidgetsOrdenador/WID_PantallaOrdenadorTriangulos` (`WidgetComponent.GetWidget` (`self.Triangulos`))))
    (if (`KismetStringLibrary.EqualEqual_StrStr` (`/Game/Widgets/WidgetsOrdenador/WID_PantallaOrdenadorTriangulos.CodigoIntroducido` _aswid_pantalla_ordenador_triangulos) (`/Game/Widgets/WidgetsOrdenador/WID_PantallaOrdenadorTriangulos.CodigoCorrecto` _aswid_pantalla_ordenador_triangulos))
      (bind _returnvalue (`GameplayStatics.GetActorOfClass` "/Game/Blueprints/Ordenador/BP_Mesilla_ordenador.BP_Mesilla_ordenador_C"))
      (`/Game/Blueprints/Ordenador/BP_Mesilla_ordenador.AbrirCajon` _returnvalue (`self.segundoNivel`))
      (bind _pwd_1 (`/Game/Widgets/WidgetsOrdenador/WID_PantallaOrdenadorTriangulos.PWD_1` _aswid_pantalla_ordenador_triangulos))
      (`TextBlock.SetColorAndOpacity` _pwd_1 (make `SlateColor` (struct :`R` 0.192751 :`G` 1.0 :`A` 1.0)))
      (`TextBlock.SetColorAndOpacity` (`/Game/Widgets/WidgetsOrdenador/WID_PantallaOrdenadorTriangulos.PWD_2` _aswid_pantalla_ordenador_triangulos) (make `SlateColor` (struct :`R` 0.192751 :`G` 1.0 :`A` 1.0)))
      (else
        (`TextBlock.SetColorAndOpacity` _pwd_1 (make `SlateColor` (struct :`R` 1.0 :`B` 0.026767 :`A` 1.0)))
        (`TextBlock.SetColorAndOpacity` (`/Game/Widgets/WidgetsOrdenador/WID_PantallaOrdenadorTriangulos.PWD_2` _aswid_pantalla_ordenador_triangulos) (make `SlateColor` (struct :`R` 1.0 :`B` 0.026767 :`A` 1.0)))
        (`KismetSystemLibrary.Delay` 2.0)
        (`TextBlock.SetColorAndOpacity` _pwd_1 (make `SlateColor` (struct :`A` 1.0)))
        (`TextBlock.SetColorAndOpacity` (`/Game/Widgets/WidgetsOrdenador/WID_PantallaOrdenadorTriangulos.PWD_2` _aswid_pantalla_ordenador_triangulos) (make `SlateColor` (struct :`A` 1.0)))))
    (elif (`KismetStringLibrary.EqualEqual_StrStr` (`/Game/Widgets/WidgetsOrdenador/WID_PantallaOrdenador.CodigoIntroducido` _aswid_pantalla_ordenador) (`self.CodigoCorrecto`))
      (bind _returnvalue_2 (`GameplayStatics.GetActorOfClass` "/Game/Blueprints/Ordenador/BP_Mesilla_ordenador.BP_Mesilla_ordenador_C"))
      (`/Game/Blueprints/Ordenador/BP_Mesilla_ordenador.AbrirCajon` _returnvalue_2 (`self.segundoNivel`))
      (bind _pwd_1_2 (`/Game/Widgets/WidgetsOrdenador/WID_PantallaOrdenador.PWD_1` _aswid_pantalla_ordenador))
      (`TextBlock.SetColorAndOpacity` _pwd_1_2 (make `SlateColor` (struct :`R` 0.192751 :`G` 1.0 :`A` 1.0)))
      (`TextBlock.SetColorAndOpacity` (`/Game/Widgets/WidgetsOrdenador/WID_PantallaOrdenador.PWD_2` _aswid_pantalla_ordenador) (make `SlateColor` (struct :`R` 0.192751 :`G` 1.0 :`A` 1.0)))
      (`TextBlock.SetColorAndOpacity` (`/Game/Widgets/WidgetsOrdenador/WID_PantallaOrdenador.PWD_3` _aswid_pantalla_ordenador) (make `SlateColor` (struct :`R` 0.192751 :`G` 1.0 :`A` 1.0)))
      (`TextBlock.SetColorAndOpacity` (`/Game/Widgets/WidgetsOrdenador/WID_PantallaOrdenador.PWD_4` _aswid_pantalla_ordenador) (make `SlateColor` (struct :`R` 0.192751 :`G` 1.0 :`A` 1.0)))
      (`TextBlock.SetText` _pwd_1_2 "O")
      (bind _pwd_2 (`/Game/Widgets/WidgetsOrdenador/WID_PantallaOrdenador.PWD_2` _aswid_pantalla_ordenador))
      (`TextBlock.SetText` _pwd_2 "P")
      (bind _pwd_3 (`/Game/Widgets/WidgetsOrdenador/WID_PantallaOrdenador.PWD_3` _aswid_pantalla_ordenador))
      (`TextBlock.SetText` _pwd_3 "E")
      (bind _pwd_4 (`/Game/Widgets/WidgetsOrdenador/WID_PantallaOrdenador.PWD_4` _aswid_pantalla_ordenador))
      (`TextBlock.SetText` _pwd_4 "N")
      (`KismetSystemLibrary.Delay` 3.0)
      (`Widget.SetVisibility` _aswid_pantalla_ordenador "Hidden")
      (bind _aswid_pantalla_ordenador_triangulos_2 (cast `/Game/Widgets/WidgetsOrdenador/WID_PantallaOrdenadorTriangulos` (`WidgetComponent.GetWidget` (`self.Triangulos`))))
      (`Widget.SetVisibility` _aswid_pantalla_ordenador_triangulos_2 "Visible")
      (set `self.Contador` 0)
      (set `self.segundoNivel` true)
      (else
        (`TextBlock.SetColorAndOpacity` _pwd_1_2 (make `SlateColor` (struct :`R` 1.0 :`B` 0.026767 :`A` 1.0)))
        (`TextBlock.SetColorAndOpacity` _pwd_2 (make `SlateColor` (struct :`R` 1.0 :`B` 0.026767 :`A` 1.0)))
        (`TextBlock.SetColorAndOpacity` _pwd_3 (make `SlateColor` (struct :`R` 1.0 :`B` 0.026767 :`A` 1.0)))
        (`TextBlock.SetColorAndOpacity` _pwd_4 (make `SlateColor` (struct :`R` 1.0 :`B` 0.026767 :`A` 1.0)))
        (`KismetSystemLibrary.Delay` 2.0)
        (`TextBlock.SetColorAndOpacity` _pwd_1_2 (make `SlateColor` (struct :`R` 0.070588 :`B` 1.0 :`A` 1.0)))
        (`TextBlock.SetColorAndOpacity` _pwd_2 (make `SlateColor` (struct :`R` 1.0 :`G` 0.098039 :`B` 0.039216 :`A` 1.0)))
        (`TextBlock.SetColorAndOpacity` _pwd_3 (make `SlateColor` (struct :`R` 0.176471 :`G` 1.0 :`A` 1.0)))
        (`TextBlock.SetColorAndOpacity` _pwd_4 (make `SlateColor` (struct :`R` 1.0 :`G` 0.019608 :`B` 0.788235 :`A` 1.0)))))))

(event `ResetMulticast`
  (params (cont :type Integer))
  ;[1 1 1] Resetea los numeros del codigo a 0
  (if (`self.segundoNivel`)
    (bind _aswid_pantalla_ordenador_triangulos (cast `/Game/Widgets/WidgetsOrdenador/WID_PantallaOrdenadorTriangulos` (`WidgetComponent.GetWidget` (`self.Triangulos`))))
    (switch `int` cont
      (:`0`
        (`TextBlock.SetText` (`/Game/Widgets/WidgetsOrdenador/WID_PantallaOrdenadorTriangulos.PWD_1` _aswid_pantalla_ordenador_triangulos) "_"))
      (:`1`
        (`TextBlock.SetText` (`/Game/Widgets/WidgetsOrdenador/WID_PantallaOrdenadorTriangulos.PWD_2` _aswid_pantalla_ordenador_triangulos) "_")))
    (else
      (bind _aswid_pantalla_ordenador (cast `/Game/Widgets/WidgetsOrdenador/WID_PantallaOrdenador` (`WidgetComponent.GetWidget` (`self.Widget`))))
      (switch `int` cont
        (:`0`
          (`TextBlock.SetText` (`/Game/Widgets/WidgetsOrdenador/WID_PantallaOrdenador.PWD_1` _aswid_pantalla_ordenador) "_"))
        (:`1`
          (`TextBlock.SetText` (`/Game/Widgets/WidgetsOrdenador/WID_PantallaOrdenador.PWD_2` _aswid_pantalla_ordenador) "_"))
        (:`2`
          (`TextBlock.SetText` (`/Game/Widgets/WidgetsOrdenador/WID_PantallaOrdenador.PWD_3` _aswid_pantalla_ordenador) "_"))
        (:`3`
          (`TextBlock.SetText` (`/Game/Widgets/WidgetsOrdenador/WID_PantallaOrdenador.PWD_4` _aswid_pantalla_ordenador) "_"))))))

(fn `UserConstructionScript`)
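; BP_VRGameMode is a multiplayer VR game mode that assigns one spectator and numbered VR players.
; After a delay on BeginPlay, the first controller possesses a spawned spectator pawn and the others possess placed VRPawns tagged with their PlayerNumber.
; For three or four players it destroys surplus pawns; the three-player branch also notifies BP_VRGameState and recolors right hands.
; ChoosePlayerStart picks the PlayerStart whose tag matches the current player count.
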(event `self.ReceiveBeginPlay`
  (bind _out_actors (`self.Out Actors`))
  (bind _output (`|GetArrayItem` _out_actors 2))
  (bind _output_2 (`|GetArrayItem` _out_actors 3))
  (bind _handright (`/Game/VRTemplate/Blueprints/VRPawn.HandRight` _output))
  (bind _handright_2 (`/Game/VRTemplate/Blueprints/VRPawn.HandRight` (`|GetArrayItem` _out_actors)))
  (bind _handright_3 (`/Game/VRTemplate/Blueprints/VRPawn.HandRight` (`|GetArrayItem` _out_actors 1)))
  ;[1 1 1] Muestra el numero introducido en el txt correspondiente
  (`KismetSystemLibrary.Delay` 2.0)
  (bind _outactors (`GameplayStatics.GetAllActorsOfClass` "/Game/Blueprints/BP_VRPlayerController.BP_VRPlayerController_C"))
  (for (_array_element _array_index) _outactors
    (if (== _array_index 0)
      (bind _returnvalue (`|SpawnActorFromClass` "/Game/Blueprints/BP_SpectatorPawn.BP_SpectatorPawn_C" (`KismetMathLibrary.MakeTransform` (0.0 0.0 0.0)) "Undefined" "MultiplyWithRoot" null null))
      (`Controller.Possess` _array_element _returnvalue)
      (else
        (bind _outactors_2 (`GameplayStatics.GetAllActorsOfClassWithTag` "/Game/VRTemplate/Blueprints/VRPawn.VRPawn_C" (`KismetStringLibrary.Conv_StringToName` (`KismetStringLibrary.Conv_IntToString` (`/Game/Blueprints/BP_VRPlayerController.PlayerNumber` _array_element)))))
        (bind _output_3 (`|GetArrayItem` _outactors_2))
        (`KismetSystemLibrary.PrintString` (`KismetSystemLibrary.GetDisplayName` _output_3))
        (`Controller.Possess` _array_element _output_3)
        (`KismetSystemLibrary.PrintString` "POSEIDO" true true (struct :`R` 1.0 :`G` 0.23878 :`B` 0.050421 :`A` 1.0) 500.0))))
  (bind _returnvalue_2 (`self.GetNumPlayers`))
  (if (== _returnvalue_2 3)
    (bind _outactors_3 (`GameplayStatics.GetAllActorsOfClassWithTag` "/Game/VRTemplate/Blueprints/VRPawn.VRPawn_C" "3"))
    (`self.K2_DestroyActor` (`|GetArrayItem` _outactors_3))
    (bind _outactors_4 (`GameplayStatics.GetAllActorsOfClassWithTag` "/Game/VRTemplate/Blueprints/VRPawn.VRPawn_C" "4"))
    (`self.K2_DestroyActor` (`|GetArrayItem` _outactors_4))
    (`KismetSystemLibrary.PrintString` "DESTRUIDO")
    (bind _asbp_vrgame_state (cast `/Game/Blueprints/BP_VRGameState` (`GameplayStatics.GetGameState`)))
    (`/Game/Blueprints/BP_VRGameState.Postit` _asbp_vrgame_state _returnvalue_2)
    (if (not (== _returnvalue_2 1))
      (switch `int` _returnvalue_2
        (:`3`
          (`PrimitiveComponent.SetMaterial` _handright_2 0 "/Game/Characters/MannequinsXR/Materials/Instances/Manny/MI_Manny_N4.MI_Manny_N4")
          (`PrimitiveComponent.SetMaterial` _handright_3 0 "/Game/Characters/MannequinsXR/Materials/Instances/Manny/MI_Manny_N9.MI_Manny_N9")
          (`self.K2_DestroyActor` _output_2)
          (`self.K2_DestroyActor` _output))
        (:`4`
          (`PrimitiveComponent.SetMaterial` _handright_2 0 "/Game/Characters/MannequinsXR/Materials/Instances/Manny/MI_Manny_N8.MI_Manny_N8")
          (`PrimitiveComponent.SetMaterial` _handright_3 0 "/Game/Characters/MannequinsXR/Materials/Instances/Manny/MI_Manny_N4.MI_Manny_N4")
          (`PrimitiveComponent.SetMaterial` _handright 0 "/Game/Characters/MannequinsXR/Materials/Instances/Manny/MI_Manny_N9.MI_Manny_N9")
          (`self.K2_DestroyActor` _output_2))
        (:`5`
          (`PrimitiveComponent.SetMaterial` _handright_2 0 "/Game/Characters/MannequinsXR/Materials/Instances/Manny/MI_Manny_N3.MI_Manny_N3")
          (`PrimitiveComponent.SetMaterial` _handright_3 0 "/Game/Characters/MannequinsXR/Materials/Instances/Manny/MI_Manny_N8.MI_Manny_N8")
          (`PrimitiveComponent.SetMaterial` _handright 0 "/Game/Characters/MannequinsXR/Materials/Instances/Manny/MI_Manny_N4.MI_Manny_N4")
          (`PrimitiveComponent.SetMaterial` (`/Game/VRTemplate/Blueprints/VRPawn.HandRight` _output_2) 0 "/Game/Characters/MannequinsXR/Materials/Instances/Manny/MI_Manny_N9.MI_Manny_N9"))))
    (elif (== _returnvalue_2 4)
      (bind _outactors_5 (`GameplayStatics.GetAllActorsOfClassWithTag` "/Game/VRTemplate/Blueprints/VRPawn.VRPawn_C" "4"))
      (`self.K2_DestroyActor` (`|GetArrayItem` _outactors_5))
      (`KismetSystemLibrary.PrintString` "DESTRUIDO2"))))

(fn `ChoosePlayerStart`
  (params (Player :type "Controller Object Reference"))
  (returns (ReturnValue :type "Actor Object Reference"))
  (bind _returnvalue (`self.GetNumPlayers`))
  (bind _outactors (`GameplayStatics.GetAllActorsOfClass` "/Script/Engine.PlayerStart"))
  (for _array_element _outactors
    (if (== _returnvalue (`KismetStringLibrary.Conv_NameToString` (`PlayerStart.PlayerStartTag` _array_element)))
      (return _array_element))))

(fn `UserConstructionScript`)
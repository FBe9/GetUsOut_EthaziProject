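; Bomb puzzle button that, on actor overlap, checks its Id against the step of OrdenCorrecto indexed by BP_Bomba's CorrectNumber.
; While the bomb's timer is above zero, a match calls Correct, changes the material and leaves the button pressed via a timeline lerp.
; A mismatch while the bomb is Looping calls Error, then animates a press and release before clearing the Clicked latch and restoring black.
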(event `self.ReceiveBeginPlay`
  ;[1 1 1] Set Location
  (bind _output_get (set `self.InitialLocation` (`SceneComponent.K2_GetComponentLocation` (`self.ButtonTop`))))
  (set `self.EndLocation` (`KismetMathLibrary.MakeVector` (.x _output_get) (.y _output_get) (- (.z _output_get) 2.5))))

(event `self.ReceiveActorBeginOverlap`
  (params (OtherActor :type "Actor Object Reference"))
  (bind _buttondown (`self.ButtonDown`))
  ;[1 1 1] ClickBotton
  (bind _returnvalue (`GameplayStatics.GetActorOfClass` "/Game/Blueprints/BombaYBoton/BP_Bomba.BP_Bomba_C"))
  (if (not (`self.Clicked`))
    (set `self.Clicked` true)
    (if (not (<= (`/Game/Blueprints/BombaYBoton/BP_Bomba.TimerBomb` _returnvalue) 0))
      (for (_array_element _array_index) (`self.OrdenCorrecto`)
        (if (== _array_index (`/Game/Blueprints/BombaYBoton/BP_Bomba.CorrectNumber` _returnvalue))
          (if (== _array_element (`self.Id`))
            (`|ExecutionSequence`
              (:`then_0`
                (`/Game/Blueprints/BombaYBoton/BP_Bomba.Correct` _returnvalue)
                (`PrimitiveComponent.SetMaterial` _buttondown 1 "/Engine/MapTemplates/Materials/BasicAsset03.BasicAsset03")
                ;[1 1 1] ButtonAnimation
                (bind (_direction _newtrack_0) (`Timeline|BottonClick` :!via `PlayFromStart`)
                  (:`Update`
                    (`SceneComponent.K2_SetWorldLocation` (`self.ButtonTop`) (`KismetMathLibrary.VLerp` (`self.InitialLocation`) (`self.EndLocation`) _newtrack_0) false false))))
              (:`then_1`
                (break)))
            (elif (`/Game/Blueprints/BombaYBoton/BP_Bomba.Looping` _returnvalue)
              (`/Game/Blueprints/BombaYBoton/BP_Bomba.Error` _returnvalue)
              (`PrimitiveComponent.SetMaterial` _buttondown 1 null)
              (bind (_direction_2 _newtrack_0_2) (`Timeline|Timeline` :!via `PlayFromStart`)
                (:`Update`
                  (`SceneComponent.K2_SetWorldLocation` (`self.ButtonTop`) (`KismetMathLibrary.VLerp` (`self.InitialLocation`) (`self.EndLocation`) _newtrack_0_2) false false))
                (:`Finished`
                  (bind (_direction_3 _newtrack_0_3) (`Timeline|Timeline_0` :!via `ReverseFromEnd`)
                    (:`Update`
                      (`SceneComponent.K2_SetWorldLocation` (`self.ButtonTop`) (`KismetMathLibrary.VLerp` (`self.InitialLocation`) (`self.EndLocation`) _newtrack_0_3) false false))
                    (:`Finished`
                      (set `self.Clicked` false)
                      (`PrimitiveComponent.SetMaterial` (`self.ButtonDown`) 1 "/Engine/EngineDebugMaterials/BlackUnlitMaterial.BlackUnlitMaterial"))))))))))))

(fn `UserConstructionScript`)
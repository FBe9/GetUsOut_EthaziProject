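; Washing machine actor for what appears to be a VR cube puzzle, with a grabbable door that reveals a puzzle cube.
; BeginPlay caches one tagged BP_Cubo_Puzle by array index and limits it to physics-only collision.
; Grabbing plays a door sound, swings the mesh open over time and restores the cube's query collision.
; UpdateLocation, uncalled here, turns a capsule by motion-controller yaw, clamped by spline point Y values.
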(event `self.ReceiveBeginPlay`
  (bind _outactors (`GameplayStatics.GetAllActorsOfClassWithTag` "/Game/Blueprints/Caja_Puzle/BP_Cubo_Puzle.BP_Cubo_Puzle_C" "2"))
  (bind _output (`|GetArrayItem` _outactors 4))
  (set `self.Cubo` _output)
  (`PrimitiveComponent.SetCollisionEnabled` (`/Game/Blueprints/Caja_Puzle/BP_Cubo_Puzle.StaticMesh` _output) "PhysicsOnly"))

(event `self.GrabComponent.OnGrabbed`
  (params (`Motion Controller` :type "MotionControllerComponent Object Reference"))
  (bind _sotano_habitacion1_washingmachine_001 (`self.Sotano_Habitacion1_WashingMachine_001`))
  (bind (_relativerotation_roll _relativerotation_pitch) (`KismetMathLibrary.BreakRotator` (`SceneComponent.RelativeRotation` _sotano_habitacion1_washingmachine_001)))
  (`GameplayStatics.PlaySoundAtLocation` "/Game/Audio/Audio_PuertaAbriendose.Audio_PuertaAbriendose" (`self.K2_GetActorLocation`) (struct) 1.0 1.0 0.0 null null null null)
  (set `self.RotacionZ` 140.0)
  (`KismetSystemLibrary.MoveComponentTo` _sotano_habitacion1_washingmachine_001 (`SceneComponent.RelativeLocation` _sotano_habitacion1_washingmachine_001) (`KismetMathLibrary.MakeRotator` _relativerotation_roll _relativerotation_pitch (`self.RotacionZ`)) false false 4.0)
  (`PrimitiveComponent.SetCollisionEnabled` (`/Game/Blueprints/Caja_Puzle/BP_Cubo_Puzle.StaticMesh` (`self.Cubo`)) "QueryAndPhysics"))

(fn `UpdateLocation`
  (bind _capsule (`self.Capsule`))
  (bind _spline (`self.Spline`))
  (bind (_returnvalue_x _returnvalue_y) (`KismetMathLibrary.BreakVector` (`SplineComponent.GetLocationAtSplinePoint` _spline 1 "Local")))
  (bind (_returnvalue_x_2 _returnvalue_y_2) (`KismetMathLibrary.BreakVector` (`SplineComponent.GetLocationAtSplinePoint` _spline 0 "Local")))
  (bind (_relativerotation_roll _relativerotation_pitch _relativerotation_yaw) (`KismetMathLibrary.BreakRotator` (`SceneComponent.RelativeRotation` _capsule)))
  (`SceneComponent.K2_SetRelativeRotation` (`self.Capsule`) (`KismetMathLibrary.MakeRotator` _relativerotation_roll _relativerotation_pitch (`KismetMathLibrary.FClamp` (+ _relativerotation_yaw (.yaw (.rotation (`KismetMathLibrary.MakeRelativeTransform` (`SceneComponent.K2_GetComponentToWorld` (`self.Motion Controller`)) (`SceneComponent.K2_GetComponentToWorld` _capsule))))) _returnvalue_y_2 _returnvalue_y)) false false))

(fn `UserConstructionScript`)
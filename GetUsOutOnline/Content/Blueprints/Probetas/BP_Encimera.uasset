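; Countertop puzzle that is solved when four coloured test tubes (BP_Probeta) each sit in their matching slot.
; Box overlaps compare material names, snap correct tubes to hard-coded positions and set per-colour flags.
; With all flags set, it plays a sound once, animates an MPCTapas parameter by timeline for the lids and disables tube collision.
; End overlaps clear flags only for BP_Cubo_Puzle actors, not tubes.
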(event `Tapar`
  (bind _mpc_tapas (`self.MPC_Tapas`))
  ;[1 1 1] Poner tapas
  (bind (_direction _newtrack_0) (`Timeline|Opacity_Change`)
    (:`Update`
      (`KismetMaterialLibrary.SetScalarParameterValue` _mpc_tapas (`|GetArrayItem` (`MaterialParameterCollection.GetScalarParameterNames` _mpc_tapas)) _newtrack_0))))

(event `ResolverProbetas`
  ;[1 1 1] En el caso de que todas las probetas esten colocados en su sitio sale la bomba
  (if (and (`self.boo_Azul`) (`self.boo_Morado`) (`self.boo_Rojo`) (`self.boo_Verde`))
    (if (not (`self.boo_Resuelto`))
      (set `self.boo_Resuelto` true)
      (`GameplayStatics.PlaySound2D` "/Engine/VREditor/Sounds/UI/Dockable_Window_Drop.Dockable_Window_Drop" 1.0 1.0 0.0 null null)
      (`self.Tapar`)
      (bind _outactors (`GameplayStatics.GetAllActorsOfClass` "/Game/Blueprints/Probetas/BP_Probeta.BP_Probeta_C"))
      (`PrimitiveComponent.SetCollisionEnabled` (`/Game/Blueprints/Probetas/BP_Probeta.StaticMesh` (`|GetArrayItem` _outactors)) "NoCollision")
      (`PrimitiveComponent.SetCollisionEnabled` (`/Game/Blueprints/Probetas/BP_Probeta.StaticMesh` (`|GetArrayItem` _outactors 1)) "NoCollision")
      (`PrimitiveComponent.SetCollisionEnabled` (`/Game/Blueprints/Probetas/BP_Probeta.StaticMesh` (`|GetArrayItem` _outactors 2)) "NoCollision")
      (`PrimitiveComponent.SetCollisionEnabled` (`/Game/Blueprints/Probetas/BP_Probeta.StaticMesh` (`|GetArrayItem` _outactors 3)) "NoCollision"))))

(event `self.Box_Azul.OnComponentEndOverlap`
  (params (OverlappedComponent :type "PrimitiveComponent Object Reference") (OtherActor :type "Actor Object Reference") (OtherComp :type "PrimitiveComponent Object Reference") (OtherBodyIndex :type Integer))
  ;[0.1233 0.7579 1] Box_Azul | Comprobación de la probeta que tiene colocada
  (cast `/Game/Blueprints/Caja_Puzle/BP_Cubo_Puzle` OtherActor)
  (set `self.boo_Azul` false))

(event `self.Box_Verde.OnComponentEndOverlap`
  (params (OverlappedComponent :type "PrimitiveComponent Object Reference") (OtherActor :type "Actor Object Reference") (OtherComp :type "PrimitiveComponent Object Reference") (OtherBodyIndex :type Integer))
  ;[0 1 0.3417] Box_Verde | Comprobación de la probeta que tiene colocada
  (cast `/Game/Blueprints/Caja_Puzle/BP_Cubo_Puzle` OtherActor)
  (set `self.boo_Verde` false))

(event `self.Box_Azul.OnComponentBeginOverlap`
  (params (OverlappedComponent :type "PrimitiveComponent Object Reference") (OtherActor :type "Actor Object Reference") (OtherComp :type "PrimitiveComponent Object Reference") (OtherBodyIndex :type Integer) (bFromSweep :type Boolean) (SweepResult :type "HitResult Structure (by ref)"))
  ;[0.1233 0.7579 1] Box_Azul | Comprobación de la probeta que tiene colocada
  (bind _asbp_probeta (cast `/Game/Blueprints/Probetas/BP_Probeta` OtherActor))
  (if (`KismetStringLibrary.EqualEqual_StrStr` (`KismetSystemLibrary.GetObjectName` (`PrimitiveComponent.GetMaterial` (`/Game/Blueprints/Probetas/BP_Probeta.StaticMesh` _asbp_probeta) 0)) "MI_ProbetaAzul")
    (`KismetSystemLibrary.PrintString` "BIEEN")
    (set `self.boo_Azul` true)
    (`self.K2_SetActorLocation` _asbp_probeta (`KismetMathLibrary.MakeVector` (`self.X_AyV`) -26.0 (`self.Z_Probetas`)) false false)
    (`self.ResolverProbetas`)
    (else
      (`KismetSystemLibrary.PrintString` "MAAL")
      (set `self.boo_Azul` false))))

(event `self.Box_Verde.OnComponentBeginOverlap`
  (params (OverlappedComponent :type "PrimitiveComponent Object Reference") (OtherActor :type "Actor Object Reference") (OtherComp :type "PrimitiveComponent Object Reference") (OtherBodyIndex :type Integer) (bFromSweep :type Boolean) (SweepResult :type "HitResult Structure (by ref)"))
  ;[0 1 0.3417] Box_Verde | Comprobación de la probeta que tiene colocada
  (bind _asbp_probeta (cast `/Game/Blueprints/Probetas/BP_Probeta` OtherActor))
  (if (`KismetStringLibrary.EqualEqual_StrStr` (`KismetSystemLibrary.GetObjectName` (`PrimitiveComponent.GetMaterial` (`/Game/Blueprints/Probetas/BP_Probeta.StaticMesh` _asbp_probeta) 0)) "MI_ProbetaVerde")
    (`KismetSystemLibrary.PrintString` "BIEEN")
    (set `self.boo_Verde` true)
    (`self.K2_SetActorLocation` _asbp_probeta (`KismetMathLibrary.MakeVector` (`self.X_AyV`) 39.0 (`self.Z_Probetas`)) false false)
    (`self.ResolverProbetas`)
    (else
      (`KismetSystemLibrary.PrintString` "MAAL")
      (set `self.boo_Verde` false))))

(event `self.Box_Morado.OnComponentEndOverlap`
  (params (OverlappedComponent :type "PrimitiveComponent Object Reference") (OtherActor :type "Actor Object Reference") (OtherComp :type "PrimitiveComponent Object Reference") (OtherBodyIndex :type Integer))
  ;[0.8441 0.1479 1] Box_Morado | Comprobación de la probeta que tiene colocada
  (cast `/Game/Blueprints/Caja_Puzle/BP_Cubo_Puzle` OtherActor)
  (set `self.boo_Morado` false))

(event `self.Box_Rojo.OnComponentEndOverlap`
  (params (OverlappedComponent :type "PrimitiveComponent Object Reference") (OtherActor :type "Actor Object Reference") (OtherComp :type "PrimitiveComponent Object Reference") (OtherBodyIndex :type Integer))
  ;[1 0.08861 0.2084] Box_Rojo | Comprobación de la probeta que tiene colocada
  (cast `/Game/Blueprints/Caja_Puzle/BP_Cubo_Puzle` OtherActor)
  (set `self.boo_Rojo` false))

(event `self.Box_Morado.OnComponentBeginOverlap`
  (params (OverlappedComponent :type "PrimitiveComponent Object Reference") (OtherActor :type "Actor Object Reference") (OtherComp :type "PrimitiveComponent Object Reference") (OtherBodyIndex :type Integer) (bFromSweep :type Boolean) (SweepResult :type "HitResult Structure (by ref)"))
  ;[0.8441 0.1479 1] Box_Morado | Comprobación de la probeta que tiene colocada
  (bind _asbp_probeta (cast `/Game/Blueprints/Probetas/BP_Probeta` OtherActor))
  (if (`KismetStringLibrary.EqualEqual_StrStr` (`KismetSystemLibrary.GetObjectName` (`PrimitiveComponent.GetMaterial` (`/Game/Blueprints/Probetas/BP_Probeta.StaticMesh` _asbp_probeta) 0)) "MI_ProbetaMorada")
    (`KismetSystemLibrary.PrintString` "BIEEN")
    (set `self.boo_Morado` true)
    (`self.K2_SetActorLocation` _asbp_probeta (`KismetMathLibrary.MakeVector` (`self.X_MyR`) -11.0 (`self.Z_Probetas`)) false false)
    (`self.ResolverProbetas`)
    (else
      (`KismetSystemLibrary.PrintString` "MAAL")
      (set `self.boo_Morado` false))))

(event `self.Box_Rojo.OnComponentBeginOverlap`
  (params (OverlappedComponent :type "PrimitiveComponent Object Reference") (OtherActor :type "Actor Object Reference") (OtherComp :type "PrimitiveComponent Object Reference") (OtherBodyIndex :type Integer) (bFromSweep :type Boolean) (SweepResult :type "HitResult Structure (by ref)"))
  ;[1 0.08861 0.2084] Box_Rojo | Comprobación de la probeta que tiene colocada
  (bind _asbp_probeta (cast `/Game/Blueprints/Probetas/BP_Probeta` OtherActor))
  (if (`KismetStringLibrary.EqualEqual_StrStr` (`KismetSystemLibrary.GetObjectName` (`PrimitiveComponent.GetMaterial` (`/Game/Blueprints/Probetas/BP_Probeta.StaticMesh` _asbp_probeta) 0)) "MI_ProbetaRoja")
    (`KismetSystemLibrary.PrintString` "BIEEN")
    (set `self.boo_Rojo` true)
    (`self.K2_SetActorLocation` _asbp_probeta (`KismetMathLibrary.MakeVector` (`self.X_MyR`) 24.0 (`self.Z_Probetas`)) false false)
    (`self.ResolverProbetas`)
    (else
      (`KismetSystemLibrary.PrintString` "MAAL")
      (set `self.boo_Rojo` false))))

(fn `UserConstructionScript`)
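; BP_Mando is a grabbable TV remote that needs two batteries before it can turn on the screen.
; A box overlap destroys each incoming BP_Pila and reveals one of the two built-in battery meshes.
; PulsarBoton works only when held with both batteries visible, playing a sound, material swap and timeline-driven button press, then calling MostrarPantalla on BP_Tele.
; Grab events toggle physics and collision on the remote's meshes.
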(event `self.GrabComponent.OnGrabbed`
  (params (`Motion Controller` :type "MotionControllerComponent Object Reference"))
  (bind _mando_mando_base_005 (`self.Mando_Mando_Base_005`))
  (`PrimitiveComponent.SetSimulatePhysics` _mando_mando_base_005 false)
  (`PrimitiveComponent.SetSimulatePhysics` (`self.Mando_Main_Button_001`) false)
  (`PrimitiveComponent.SetSimulatePhysics` (`self.Mando_Mando_Base_Tapa_001`) false)
  (`PrimitiveComponent.SetSimulatePhysics` (`self.Mando_Pilas_001`) false)
  (`PrimitiveComponent.SetSimulatePhysics` (`self.Mando_Pilas_002`) false)
  (`PrimitiveComponent.SetCollisionEnabled` _mando_mando_base_005 "NoCollision")
  (`PrimitiveComponent.SetCollisionEnabled` (`self.Mando_Main_Button_001`) "NoCollision")
  (`PrimitiveComponent.SetCollisionEnabled` (`self.Mando_Mando_Base_Tapa_001`) "NoCollision")
  (`PrimitiveComponent.SetCollisionEnabled` (`self.Mando_Pilas_001`) "NoCollision")
  (`PrimitiveComponent.SetCollisionEnabled` (`self.Mando_Pilas_002`) "NoCollision")
  (set `self.grabed` true))

(event `self.GrabComponent.OnDropped`
  (bind _mando_mando_base_005 (`self.Mando_Mando_Base_005`))
  (`PrimitiveComponent.SetSimulatePhysics` _mando_mando_base_005 true)
  (`PrimitiveComponent.SetCollisionEnabled` _mando_mando_base_005 "QueryAndPhysics")
  (set `self.grabed` false))

(event `PulsarBoton`
  ;[1 1 1] ToDo: Animación de boton bajando y sonido de pulsación
  (if (and (`SceneComponent.bVisible` (`self.Mando_Pilas_001`)) (`SceneComponent.bVisible` (`self.Mando_Pilas_002`)) (`self.grabed`))
    (`GameplayStatics.PlaySound2D` "/Game/Audio/Audio_PulsarBoton_Mando.Audio_PulsarBoton_Mando" 1.0 1.0 0.0 null null)
    (`PrimitiveComponent.SetMaterial` (`self.Mando_Mando_Base_005`) 6 "/Engine/EngineDebugMaterials/TerrainCollisionMaterial.TerrainCollisionMaterial")
    (bind (_direction _newtrack_0) (`Timeline|Timeline`)
      (:`Update`
        (`KismetSystemLibrary.MoveComponentTo` (`self.Mando_Main_Button_001`) (`KismetMathLibrary.MakeVector` 0.0 0.0 _newtrack_0) (struct) false false 0.0))
      (:`Finished`
        (`PrimitiveComponent.SetMaterial` (`self.Mando_Mando_Base_005`) 6 "/Engine/BufferVisualization/WorldNormal.WorldNormal")
        (`KismetSystemLibrary.MoveComponentTo` (`self.Mando_Main_Button_001`) (0.0 0.0 0.0) (struct) false false 0.3)
        (bind _returnvalue (`GameplayStatics.GetActorOfClass` "/Game/Blueprints/Mando_Pilas/BP_Tele.BP_Tele_C"))
        (`/Game/Blueprints/Mando_Pilas/BP_Tele.MostrarPantalla` _returnvalue)))))

(event `self.Box.OnComponentBeginOverlap`
  (params (OverlappedComponent :type "PrimitiveComponent Object Reference") (OtherActor :type "Actor Object Reference") (OtherComp :type "PrimitiveComponent Object Reference") (OtherBodyIndex :type Integer) (bFromSweep :type Boolean) (SweepResult :type "HitResult Structure (by ref)"))
  ;[1 1 1] Comprobar Pilas en posición
  (bind _asbp_pila (cast `/Game/Blueprints/Mando_Pilas/BP_Pila` OtherActor))
  (`self.K2_DestroyActor` _asbp_pila)
  (if (`SceneComponent.bVisible` (`self.Mando_Pilas_001`))
    (`SceneComponent.SetVisibility` (`self.Mando_Pilas_002`) true false)
    (else
      (`SceneComponent.SetVisibility` (`self.Mando_Pilas_001`) true false))))

(fn `UserConstructionScript`)
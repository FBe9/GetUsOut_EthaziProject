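; VR nightstand for the cube-and-balance puzzle, with grabbable sliding drawers, one locked until AbrirCajon unlocks it and slides the upper drawer to a set position with sound.
; While grabbed, looping timers move each capsule along local Y with the motion controller, clamped between two spline points.
; A tagged BP_Cubo_Puzle has query collision disabled at BeginPlay, restored by grabbing the unlocked drawer or by AbrirCajon.
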(event `AbrirCajon`
  (bind _v001_mesilla_cajon_cajon_arriba (`self.v001_Mesilla_Cajon_Cajon_Arriba`))
  (bind (_relativelocation_x _relativelocation_y _relativelocation_z) (`KismetMathLibrary.BreakVector` (`SceneComponent.RelativeLocation` _v001_mesilla_cajon_cajon_arriba)))
  (set `self.Abierto` true)
  (`GameplayStatics.PlaySound2D` "/Engine/VREditor/Sounds/VR_negative.VR_negative" 1.0 1.0 0.0 null null)
  (`PrimitiveComponent.SetCollisionEnabled` (`/Game/Blueprints/Caja_Puzle/BP_Cubo_Puzle.StaticMesh` (`self.As BP Cubo Puzle`)) "QueryAndPhysics")
  (`KismetSystemLibrary.MoveComponentTo` _v001_mesilla_cajon_cajon_arriba (`KismetMathLibrary.MakeVector` _relativelocation_x 5.0 _relativelocation_z) (`SceneComponent.RelativeRotation` _v001_mesilla_cajon_cajon_arriba) false false 1.0)
  (`GameplayStatics.PlaySound2D` "/Game/Audio/AudiosPshicopat/segundo-paso.segundo-paso" 1.0 1.0 0.0 null null))

(event `self.GrabComponent1.OnGrabbed`
  (params (`Motion Controller` :type "MotionControllerComponent Object Reference"))
  (if (`self.Abierto`)
    (set `self.Motion Controller_0` `Motion Controller`)
    (bind _returnvalue (`KismetSystemLibrary.K2_SetTimer` null "UpdateLocation_0" 0.01 true))
    (set `self.Timer_0` _returnvalue)))

(event `self.GrabComponent.OnGrabbed`
  (params (`Motion Controller` :type "MotionControllerComponent Object Reference"))
  (`GameplayStatics.PlaySoundAtLocation` "/Engine/VREditor/Sounds/VR_grab.VR_grab" (`SceneComponent.K2_GetComponentLocation` (`self.GrabComponent`)) (struct) 1.0 1.0 0.0 null null null null)
  (set `self.Motion Controller` `Motion Controller`)
  (bind _returnvalue (`KismetSystemLibrary.K2_SetTimer` null "UpdateLocation" 0.01 true))
  (set `self.Timer` _returnvalue)
  (`PrimitiveComponent.SetCollisionEnabled` (`/Game/Blueprints/Caja_Puzle/BP_Cubo_Puzle.StaticMesh` (`self.As BP Cubo Puzle`)) "QueryAndPhysics"))

(event `self.GrabComponent1.OnDropped`
  (if true
    (`KismetSystemLibrary.K2_ClearAndInvalidateTimerHandle` (`self.Timer_0`))
    (set `self.Motion Controller_0` null)))

(event `self.GrabComponent.OnDropped`
  (`KismetSystemLibrary.K2_ClearAndInvalidateTimerHandle` (`self.Timer`))
  (set `self.Motion Controller` null))

(event `self.ReceiveBeginPlay`
  (bind _outactors (`GameplayStatics.GetAllActorsOfClassWithTag` "/Game/Blueprints/Caja_Puzle/BP_Cubo_Puzle.BP_Cubo_Puzle_C" "3"))
  (bind _output_get (set `self.As BP Cubo Puzle` (`|GetArrayItem` _outactors 3)))
  (`PrimitiveComponent.SetCollisionEnabled` (`/Game/Blueprints/Caja_Puzle/BP_Cubo_Puzle.StaticMesh` _output_get) "PhysicsOnly"))

(fn `UpdateLocation`
  (locals (NewLocalVar :type "Rotator Structure" :default (struct)))
  (bind _capsule (`self.Capsule`))
  (bind _spline (`self.Spline`))
  (bind (_returnvalue_x _returnvalue_y) (`KismetMathLibrary.BreakVector` (`SplineComponent.GetLocationAtSplinePoint` _spline 1 "Local")))
  (bind (_returnvalue_x_2 _returnvalue_y_2) (`KismetMathLibrary.BreakVector` (`SplineComponent.GetLocationAtSplinePoint` _spline 0 "Local")))
  (bind (_relativelocation_x _relativelocation_y _relativelocation_z) (`KismetMathLibrary.BreakVector` (`SceneComponent.RelativeLocation` _capsule)))
  (`SceneComponent.K2_SetRelativeLocation` _capsule (`KismetMathLibrary.MakeVector` _relativelocation_x (`KismetMathLibrary.FClamp` (+ _relativelocation_y (.y (.location (`KismetMathLibrary.MakeRelativeTransform` (`SceneComponent.K2_GetComponentToWorld` (`self.Motion Controller`)) (`SceneComponent.K2_GetComponentToWorld` _capsule))))) _returnvalue_y_2 _returnvalue_y) _relativelocation_z) false false))

(fn `UpdateLocation_0`
  (locals (NewLocalVar :type "Rotator Structure" :default (struct)))
  (bind _capsule1 (`self.Capsule1`))
  (bind _spline (`self.Spline`))
  (bind (_returnvalue_x _returnvalue_y) (`KismetMathLibrary.BreakVector` (`SplineComponent.GetLocationAtSplinePoint` _spline 1 "Local")))
  (bind (_returnvalue_x_2 _returnvalue_y_2) (`KismetMathLibrary.BreakVector` (`SplineComponent.GetLocationAtSplinePoint` _spline 0 "Local")))
  (bind (_relativelocation_x _relativelocation_y _relativelocation_z) (`KismetMathLibrary.BreakVector` (`SceneComponent.RelativeLocation` _capsule1)))
  (`SceneComponent.K2_SetRelativeLocation` _capsule1 (`KismetMathLibrary.MakeVector` _relativelocation_x (`KismetMathLibrary.FClamp` (+ _relativelocation_y (.y (.location (`KismetMathLibrary.MakeRelativeTransform` (`SceneComponent.K2_GetComponentToWorld` (`self.Motion Controller_0`)) (`SceneComponent.K2_GetComponentToWorld` _capsule1))))) _returnvalue_y_2 _returnvalue_y) _relativelocation_z) false false))

(fn `UserConstructionScript`)